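; Linked portal actor (传送门) that shows a live view through its partner and teleports FirstPersonCharacters, with A/B materials and render targets chosen by PortalA.
; Each tick mirrors the player camera onto the partner's scene capture, adjusts its near clip plane and resizes the render target to the viewport.
; Overlapping characters switch to a portalPawn collision profile.
; Crossing the plane while moving inward teleports them, remapping position, view and velocity to the partner.
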(event OnComponentBeginOverlap(传送门内)
  (params (OverlappedComponent :type Primitive%20Component%20Object%20Reference) (OtherActor :type Actor%20Object%20Reference) (OtherComp :type Primitive%20Component%20Object%20Reference) (OtherBodyIndex :type Integer) (bFromSweep :type Boolean) (SweepResult :type Hit%20Result%20Structure%20%28by%20ref%29)))

(event OnComponentEndOverlap(传送门内)
  (params (OverlappedComponent :type Primitive%20Component%20Object%20Reference) (OtherActor :type Actor%20Object%20Reference) (OtherComp :type Primitive%20Component%20Object%20Reference) (OtherBodyIndex :type Integer)))

(event EventBeginPlay)

(event EventTick
  (params (DeltaSeconds :type Float%20%28single-precision%29))
  (bind _returnvalue (Viewport|GetViewportSize))
  (bind _returnvalue_2 (Game|GetPlayerCameraManager 0))
  (bind _门户纹理质量 (Variables|Default|Get门户纹理质量))
  (bind _backfacingscene (Variables|Default|GetBackFacingScene))
  (bind _returnvalue_3 (Transformation|GetWorldTransform _backfacingscene))
  (bind _transformcomponent (Variables|/Script/Engine.PlayerCameraManager|GetTransformComponent _returnvalue_2))
  (bind _returnvalue_4 (Transformation|GetWorldTransform _transformcomponent))
  (bind _returnvalue_5 (Class|KismetMathLibrary|ConvertTransformtoRelative _returnvalue_3 (Math|Transform|MakeTransform (.location _returnvalue_4) (.rotation _returnvalue_4) (.scale _returnvalue_4))))
  (bind _链接的传送门 (Variables|Default|Get链接的传送门)
    (:then
      (Transformation|SetRelativeLocationAndRotation (Variables|BP_传送门_C|GetSceneCaptureComponent2D _链接的传送门) (.location _returnvalue_5) (.rotation _returnvalue_5) false false)
      (Utilities|FlowControl|Sequence
        (:then_0
          ;[1 1 1] 设置传送门内渲染纹理
          (Rendering|ResizeRenderTarget2D (Variables|/Script/Engine.SceneCaptureComponent2D|GetTextureTarget (Variables|Default|GetSceneCaptureComponent2D)) (Math|Float|Truncate (* (.x _returnvalue) _门户纹理质量)) (Math|Float|Truncate (* (.y _returnvalue) _门户纹理质量)))
          (bind _链接的传送门_2 (Variables|Default|Get链接的传送门)
            (:then
              (Variables|/Script/Engine.SceneCaptureComponent2D|SetCustomNearClippingPlane (Variables|BP_传送门_C|GetSceneCaptureComponent2D _链接的传送门_2) (+ (Math|Vector|Distance(Vector) (Transformation|GetWorldLocation (Variables|/Script/Engine.PlayerCameraManager|GetTransformComponent (Game|GetPlayerCameraManager 0))) (Transformation|GetActorLocation)) 1.0)))
            (:else)))
        (:then_1
          ;[1 1 1] 角色传送检测
          (for _array_element (Variables|Default|Get接触传送门的玩家)
            (bind _结果 (CallFunction|玩家是否应该传送 _array_element))
            (if _结果
              (CallFunction|进行传送 _array_element))))))
    (:else)))

(event Collision|EventActorBeginOverlap
  (params (OtherActor :type Actor%20Object%20Reference))
  (bind _asfirst_person_character (Utilities|Casting|CastToFirstPersonCharacter OtherActor))
  (Utilities|FlowControl|DoOnce false
    (:Completed
      (bind _链接的传送门 (Variables|Default|Get链接的传送门)
        (:then
          (if (Utilities|IsValid _链接的传送门)
            (bind _returnvalue (Utilities|Array|AddUnique (Variables|Default|Get接触传送门的玩家) _asfirst_person_character))
            (if (!= _returnvalue -1)
              (Collision|SetCollisionProfileName (Variables|/Script/Engine.Character|GetCapsuleComponent _asfirst_person_character) "portalPawn" true :!class /Script/Engine.PrimitiveComponent))))
        (:else)))))

(event Collision|EventActorEndOverlap
  (params (OtherActor :type Actor%20Object%20Reference))
  (bind _asfirst_person_character (Utilities|Casting|CastToFirstPersonCharacter OtherActor))
  (Utilities|Array|RemoveItem (Variables|Default|Get接触传送门的玩家) _asfirst_person_character)
  (Collision|SetCollisionProfileName (Variables|/Script/Engine.Character|GetCapsuleComponent _asfirst_person_character) "Pawn" true :!class /Script/Engine.PrimitiveComponent)
  (Utilities|FlowControl|DoOnce false) ; enters at Reset
)

(fn ConstructionScript
  (Rendering|Material|SetMaterial (Variables|Default|Get传送门内) 0 (select (Variables|Default|GetPortalA) "/Game/Portal/Material/RenderTarget/传送门内部_A.传送门内部_A" "/Game/Portal/Material/RenderTarget/传送门内部_B.传送门内部_B"))
  (Rendering|Material|SetMaterial (Variables|Default|Get传送门) 0 (select (Variables|Default|GetPortalA) "/Game/Portal/Material/Boarder/M_PortalRingA.M_PortalRingA" "/Game/Portal/Material/Boarder/M_PortalRingB.M_PortalRingB"))
  (Variables|/Script/Engine.SceneCaptureComponent2D|SetTextureTarget (Variables|Default|GetSceneCaptureComponent2D) (select (not (Variables|Default|GetPortalA)) "/Game/Portal/Material/RenderTarget/PortalRenderTargetA.PortalRenderTargetA" "/Game/Portal/Material/RenderTarget/PortalRenderTargetB.PortalRenderTargetB")))

(fn 链接传送门
  (params (portal :type BP%20传送门%20Object%20Reference) (A :type Boolean))
  (Variables|Default|Set链接的传送门 portal)
  (Utilities|IsValid 0))

(fn 玩家是否应该传送
  (params (玩家 :type First%20Person%20Character%20Object%20Reference))
  (return (and (<= (Math|Vector|DotProduct (Math|Vector|Normalize (- (+ (Transformation|GetActorLocation 玩家) (+ (Transformation|GetVelocity 玩家) (Utilities|Time|GetWorldDeltaSeconds))) (Transformation|GetActorLocation))) (Transformation|GetActorForwardVector)) 0.0) (< (Math|Vector|DotProduct (Math|Vector|Normalize (Class|Pawn|GetLastMovementInputVector 玩家)) (Transformation|GetActorForwardVector)) 0.0))))

(fn 进行传送
  (params (玩家 :type First%20Person%20Character%20Object%20Reference))
  (bind _backfacingscene (Variables|Default|GetBackFacingScene))
  (bind _链接的传送门 (Variables|Default|Get链接的传送门))
  (bind _returnvalue (Transformation|GetActorTransform _链接的传送门))
  (bind _returnvalue_2 (Transformation|GetWorldTransform _backfacingscene))
  (bind _fps_camera (Variables|/Game/VFX_SciFi_Muzzle_And_Impact_Pack_1/Example_Content/DemoContent/Blueprints/Character/FirstPersonCharacter.FirstPersonCharacter_C|GetFPS_Camera 玩家))
  (bind _returnvalue_3 (Transformation|GetWorldTransform _fps_camera))
  (bind _returnvalue_4 (Class|KismetMathLibrary|ConvertTransformtoRelative _returnvalue_2 _returnvalue_3))
  (bind _returnvalue_5 (Math|Transform|ComposeTransforms _returnvalue_4 _returnvalue))
  (bind (_roll _pitch _yaw) (Math|Rotator|BreakRotator (.rotation _returnvalue_5)))
  (LocalVariables|Set变换方向 (Math|Transform|InverseTransformDirection (Transformation|GetActorTransform 玩家) (Transformation|GetVelocity 玩家)))
  (Transformation|SetActorLocation 玩家 (+ (- (.location _returnvalue_5) (Variables|/Script/Engine.SceneComponent|GetRelativeLocation (Variables|/Game/VFX_SciFi_Muzzle_And_Impact_Pack_1/Example_Content/DemoContent/Blueprints/Character/FirstPersonCharacter.FirstPersonCharacter_C|GetFPS_Camera 玩家))) (* (Transformation|GetActorForwardVector (Variables|Default|Get链接的传送门)) 1e+01)) false true)
  (Pawn|SetControlRotation (Pawn|GetController 玩家) (Math|Rotator|MakeRotator 0.0 _pitch _yaw))
  (Variables|/Script/Engine.MovementComponent|SetVelocity (Pawn|GetMovementComponent 玩家) (Math|Transform|TransformDirection (Math|Transform|MakeTransform (Transformation|GetActorLocation 玩家) (Pawn|GetControlRotation (Pawn|GetController 玩家) :!class /Script/Engine.Controller)) (LocalVariables|Get变换方向))))