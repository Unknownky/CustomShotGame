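; Player controller for the Antize Kit systems, tying chat, team IDs, player name tags, emotes and a debug HUD together.
; BPChatComponent handles chat, player list, PlayerID and team data; authority-gated refresh events push IDs to the local debug HUD.
; Interface messages for name tag, level, username, emote and key requests mostly forward to the controlled pawn, while several others are stubs.
; Up/Down keys change player level for testing.
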(event Custom|Client_RefreshDebugHUD
  (params (RefreshPlayerID? :type Boolean) (PlayerID :type Integer) (TeamID :type Integer) (ColorID :type Integer))
  (bind _debughudref (Variables|Spawn|GetDebugHUDRef))
  ;[1 1 1] (Client) Refresh HUD
  (Utilities|IsValid (Variables|Spawn|GetDebugHUDRef)
    (:Is%20Valid
      (if RefreshPlayerID?
        (Default|RefreshPlayerID _debughudref PlayerID)
        (else
          (Default|RefreshTeamID _debughudref TeamID ColorID))))))

(event EventBeginPlay
  ;[1 1 1] Constructeur Create Widgets (Delay on chat, be sure to have PlayerID)
  (|CallParentFunction)
  (Variables|/Game/AntizeKitSystem/AntizeSystems/ChatSystem/Blueprints/BP_ChatComponent.BP_ChatComponent_C|SetControllerRef (Variables|Default|GetBP_ChatComponent) self)
  ;;[1 1 1] Only on local player
  (if (Pawn|IsLocalPlayerController)
    (bind _returnvalue (UserInterface|CreateWidget "/Game/AntizeKitSystem/Demo/Widgets/W_DebugHUD.W_DebugHUD_C" self))
    (Utilities|IsValid _returnvalue
      (:Is%20Valid
        (bind _output_get (Variables|Spawn|SetDebugHUDRef _returnvalue))
        (UserInterface|Viewport|AddtoViewport _output_get 0)))))

(event EventMSGSetTeamID
  (params (Team_ID :type Integer) (Color_ID :type Integer))
  ;[1 1 1] Set TeamID
  (Default|ServerSetTeamID (Variables|Default|GetBP_ChatComponent) Team_ID Color_ID))

(event EventMSGRefreshPlayerID
  ;[1 1 1] (Server->Client) Refresh PlayerID, TeamID & ColorID on debug HUD
  (Networking|SwitchHasAuthority
    (:Authority
      (CallFunction|ClientRefreshDebugHUD true (Variables|/Game/AntizeKitSystem/AntizeSystems/ChatSystem/Blueprints/BP_ChatComponent.BP_ChatComponent_C|GetPlayerID (Variables|Default|GetBP_ChatComponent))))))

(event EventMSGRefreshTeamID
  (bind _bp_chatcomponent (Variables|Default|GetBP_ChatComponent))
  ;[1 1 1] (Server->Client) Refresh PlayerID, TeamID & ColorID on debug HUD
  (Networking|SwitchHasAuthority
    (:Authority
      (CallFunction|ClientRefreshDebugHUD false 0 (Variables|/Game/AntizeKitSystem/AntizeSystems/ChatSystem/Blueprints/BP_ChatComponent.BP_ChatComponent_C|GetTeamID _bp_chatcomponent) (Variables|/Game/AntizeKitSystem/AntizeSystems/ChatSystem/Blueprints/BP_ChatComponent.BP_ChatComponent_C|GetColorID _bp_chatcomponent)))))

(event Input|KeyboardEvents|Up
  (params (Key :type Key%20Structure))
  ;[1 0 0] Only for test
  (:Pressed
    (bind (_playernamecomponentref _actorref) (Utilities|GetActorandPlayerName)
      (:Is%20Valid
        (Default|ServerLevelUp _playernamecomponentref _actorref)))))

(event Input|KeyboardEvents|Down
  (params (Key :type Key%20Structure))
  ;[1 0 0] Only for test
  (:Pressed
    (bind (_playernamecomponentref _actorref) (Utilities|GetActorandPlayerName)
      (:Is%20Valid
        (Default|ServerLevelDown _playernamecomponentref _actorref)))))

(event EventMSGPlayEmote
  (params (EmoteToPlay :type E_Emote%20Enum :default "NewEnumerator0"))
  (bind _returnvalue (Pawn|GetControlledPawn))
  ;[1 1 1] Play emote
  (Utilities|IsValid _returnvalue
    (:Is%20Valid
      (Class|BPAntizeChatInterface|MSGPlayEmote(Message) _returnvalue EmoteToPlay))))

(event EventMSGNewMessage
  (params (Received? :type Boolean) (MessageData :type S%20Message%20Data%20Structure))
  ;[1 1 1] Received or Send a Message
  (Default|OnNewMessage (Variables|Default|GetBP_ChatComponent) Received? MessageData))

(event Input|KeyboardEvents|Enter
  (params (Key :type Key%20Structure))
  ;[1 1 1] Open Close Chat and player list
  (:Pressed
    (Default|OpenChat (Variables|Default|GetBP_ChatComponent))))

(event Input|KeyboardEvents|P
  (params (Key :type Key%20Structure))
  ;[1 1 1] Open Close Chat and player list
  (:Pressed
    (Default|OpenPlayerList (Variables|Default|GetBP_ChatComponent))))

(event EventMSGChangeGameplaySetting
  (params (Setting :type E_TemplateUI%20Enum :default "NewEnumerator0") (Index :type Integer) (Value :type Float%20%28single-precision%29))
  (switch Utilities|FlowControl|Switch|SwitchonE_TemplateUI Setting))

(fn ConstructionScript)

(fn GetCurrentState
  (return (select (and (Variables|PlayerName|GetIsVOIP?) (Variables|PlayerName|GetIsWrite?)) "NewEnumerator3" (select (Variables|PlayerName|GetIsVOIP?) "NewEnumerator1" (select (Variables|PlayerName|GetIsWrite?) "NewEnumerator2" "NewEnumerator0")))))

(fn MSGAntizeGetPlayerID
  (return (Variables|/Game/AntizeKitSystem/AntizeSystems/ChatSystem/Blueprints/BP_ChatComponent.BP_ChatComponent_C|GetPlayerID (Variables|Default|GetBP_ChatComponent))))

(fn MSGAntizePNGetLevel
  (bind _returnvalue (Pawn|GetControlledPawn))
  (Utilities|IsValid _returnvalue
    (:Is%20Valid
      (bind _actuallevel (Class|BPAntizePlayerNameInterface|MSGAntizePNGetLevel(Message) _returnvalue))
      (return _actuallevel))
    (:Is%20Not%20Valid
      (return 0))))

(fn MSGAntizePNGetPlayerNameComponent
  (bind _playernamecomponentref (Utilities|GetActorandPlayerName)
    (:Is%20Valid
      (return _playernamecomponentref))
    (:Is%20Not%20Valid
      (return 0))))

(fn MSGAntizePNGetViewLocation
  (bind _returnvalue (Pawn|GetControlledPawn))
  (Utilities|IsValid _returnvalue
    (:Is%20Valid
      (bind _viewlocation (Class|BPAntizePlayerNameInterface|MSGAntizePNGetViewLocation(Message) _returnvalue))
      (return _viewlocation))
    (:Is%20Not%20Valid
      (return "0, 0, 0"))))

(fn MSGAntizePNGetWidgetRef
  (bind _returnvalue (Pawn|GetControlledPawn))
  (Utilities|IsValid _returnvalue
    (:Is%20Valid
      (bind _widgetcomponentref (Class|BPAntizePlayerNameInterface|MSGAntizePNGetWidgetRef(Message) _returnvalue))
      (return _widgetcomponentref))
    (:Is%20Not%20Valid
      (return 0))))

(fn MSGAntizePNTrytoInisitalize
  (bind _returnvalue (Pawn|GetControlledPawn))
  (Utilities|IsValid _returnvalue
    (:Is%20Valid
      (bind _return (Class|BPAntizePlayerNameInterface|MSGAntizePNTrytoInisitalize(Message) _returnvalue))
      (return _return))))

(fn MSGGetConnectedPlayers
  (return 0))

(fn MSGGetIsPlayer
  (return false))

(fn MSGGetSave
  (return 0))

(fn MSGGetSavefromSlot
  (params (RefreshSlot? :type Boolean) (NewSlotName :type String))
  (return 0))

(fn MSGGetTeamID
  (bind _bp_chatcomponent (Variables|Default|GetBP_ChatComponent))
  (return (Variables|/Game/AntizeKitSystem/AntizeSystems/ChatSystem/Blueprints/BP_ChatComponent.BP_ChatComponent_C|GetTeamID _bp_chatcomponent) (Variables|/Game/AntizeKitSystem/AntizeSystems/ChatSystem/Blueprints/BP_ChatComponent.BP_ChatComponent_C|GetColorID _bp_chatcomponent)))

(fn MSGGetUsername
  (bind _returnvalue (Pawn|GetControlledPawn))
  (Utilities|IsValid _returnvalue
    (:Is%20Valid
      (bind (_success_ _username) (Class|BPAntizeChatInterface|MSGGetUsername(Message) _returnvalue))
      (return _success_ _username))
    (:Is%20Not%20Valid
      (return false "No pawn found (You must try again)"))))

(fn MSGIsKeyEditing
  (return false))

(fn MSGPingGetActorType
  (return "NewEnumerator1"))

(fn MSGPingGetPingTexture
  (return "/Game/AntizeKitSystem/AntizeSystems/SimplePingSystem/Textures/T_PingOver.T_PingOver"))

(fn MSGRefreshSaveRef
  (params (NewSaveRef :type BP%20Save%20Inventory%20Object%20Reference))
  (return false))

(fn MSGRequestKey
  (params (Action? :type Boolean) (ActionName :type E_TemplateControlAction%20Enum :default "NewEnumerator0") (AxisName :type E_TemplateControlAxis%20Enum :default "NewEnumerator0"))
  (bind _returnvalue (Pawn|GetControlledPawn))
  (Utilities|IsValid _returnvalue
    (:Is%20Valid
      (bind _mykey (Class|BPAntizeMenuInterface|MSGRequestKey(Message) _returnvalue Action? ActionName AxisName))
      (return _mykey))
    (:Is%20Not%20Valid
      (return ""))))

(fn MSGRequestPlayerID
  (return 0 false))