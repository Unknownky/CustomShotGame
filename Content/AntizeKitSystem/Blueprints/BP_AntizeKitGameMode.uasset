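; BP_AntizeKitGameMode is the AntizeKit GameMode, tracking connected players, teams, difficulty, destroyed loot and player IDs.
; On BeginPlay it applies saved doors immediately, then after a short delay checks for duplicate names and applies world loot.
; Login and logout maintain the player array used for system messages and ping removal.
; MSG functions expose players, destroyed loot, saved doors and ID requests, with the rest left as default stubs.
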(event Custom|RemoveSystemPing
  ;[1 1 1] Remove all ping system
  (CallFunction|RemovePingSystem (Variables|General|GetConnectedPlayers) true -1)
  (Utilities|Array|Clear (Variables|PingSystem|GetActualRandomPing)))

(event Custom|SendsSystemMessageToPlayers
  (params (Message :type Text))
  ;[1 1 1] Sends a system message to players
  (CallFunction|SendSystemMessagetoPlayers (Variables|General|GetConnectedPlayers) Message))

(event Custom|ChangeDifficulty
  (params (NewDifficulty :type E_Difficulty%20Enum :default "NewEnumerator0"))
  ;[1 1 1] Difficulty changed (Exemple)
  (Variables|MenuSystem|SetCurrentDifficulty NewDifficulty))

(event EventBeginPlay
  ;[1 1 1] Constructor
  ;;[1 1 1] Loading of saved doors (Don't set a delay before)
  (CallFunction|ApplyDoorWorld)
  (Utilities|FlowControl|Delay 0.2)
  (CallFunction|CheckforDuplicateName)
  (CallFunction|ApplyLootWorld))

(event EventPostLogin
  (params (NewPlayer :type Player%20Controller%20Object%20Reference))
  ;[1 1 1] On new player - Add player to PlayersConnected array
  (Utilities|IsValid NewPlayer
    (:Is%20Valid
      (Utilities|Array|AddUnique (Variables|General|GetConnectedPlayers) NewPlayer))))

(event EventOnLogout
  (params (ExitingController :type Controller%20Object%20Reference))
  ;[1 1 1] On player left - Remove player from PlayersConnected array
  (Utilities|Array|RemoveItem (Variables|General|GetConnectedPlayers) ExitingController))

(event EventMSGAddDestroyedLoot
  (params (LootID :type Integer))
  ;[1 1 1] Add loot ID in the destroyed array
  (bind _outlootdestroyed (CallFunction|AddDestroyedLoot (Variables|InventorySystem|GetLootDestroyed) LootID))
  (Variables|InventorySystem|SetLootDestroyed _outlootdestroyed))

(event EventMSGPingJoinTeam
  (params (PlayerRef :type Controller%20Object%20Reference) (OldTeamID :type Integer) (ToTeamID :type Integer))
  ;[1 1 1] Join Team receveid
  (bind _newteam (CallFunction|JoinTeam PlayerRef OldTeamID ToTeamID (Variables|PingSystem|GetAllTeam)))
  (Variables|PingSystem|SetAllTeam _newteam))

(fn ConstructionScript)

(fn MSGDoorGetCamera
  (return 0))

(fn MSGGetCamera
  (return 0))

(fn MSGGetConnectedPlayers
  (return (Variables|General|GetConnectedPlayers)))

(fn MSGGetDamageLocation
  (return "0, 0, 0"))

(fn MSGGetDestroyedLoot
  (return (Variables|InventorySystem|GetLootDestroyed)))

(fn MSGGetDoorSaved
  (bind _doorsaved (CallFunction|GetDoorWorld))
  (return _doorsaved))

(fn MSGGetDropComponent
  (return 0))

(fn MSGGetInventory
  (return 0))

(fn MSGGetIsPlayer
  (return false))

(fn MSGGetTeamID
  (return 0 0))

(fn MSGGetUsername
  (return false ""))

(fn MSGGetWeaponPlayerComponent
  (return 0 0))

(fn MSGPingGetActorType
  (return "NewEnumerator0"))

(fn MSGPingGetPingTexture
  (return 0))

(fn MSGRequestPlayerID
  (bind _playerid (CallFunction|DoRequestPlayerID (Variables|General|GetUniquePlayerID)))
  (return _playerid true))