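; BP_Loot is a world pickup actor holding an item stack for the inventory system.
; Construction assigns a random save ID and builds mesh, materials and offsets from the DT_Item row, rerun when ItemOnLoot replicates.
; Interaction messages toggle the pickup prompt, update the remaining amount, or have the player's BP_InventoryComponent server-destroy emptied loot.
; DoSaveLoot updates or appends its save entry by LootID unless IgnoreSaving is set.
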(event Custom|RefreshInteract
  (params (Key :type Text) (Amount :type Integer))
  ;[1 1 1] Refresh interact text
  (bind _returnvalue (Utilities|GetDataTableRow "/Game/AntizeKitSystem/AntizeSystems/InventorySystem/Logics/DT_Item.DT_Item" (.RowName (Utilities|Struct|BreakDataTableRowHandle (Utilities|Struct|BreakS_InventorySlot (Variables|Setting|GetItemOnLoot)))))
    (:then
      (bind _asw_interact (Utilities|Casting|CastToW_Interact (UserInterface|GetUserWidgetObject (Variables|Default|GetWidget))))
      (Default|UpdateInteract _asw_interact Key (Utilities|Text|FormatText "to pick-up ({Amount} {Name})" Amount (Variables|Spawn|GetItemName)) (Utilities|Struct|BreakS_Item _returnvalue) true))))

(event EventBeginPlay
  ;[1 1 1] Hide debug text
  (Rendering|SetVisibility (Variables|Default|GetTextRender) false false)
  (bind _returnvalue (Utilities|GetDataTableRow "/Game/AntizeKitSystem/AntizeSystems/InventorySystem/Logics/DT_Item.DT_Item" (.RowName (Utilities|Struct|BreakDataTableRowHandle (Utilities|Struct|BreakS_InventorySlot (Variables|Setting|GetItemOnLoot)))))
    (:then
      (Variables|Spawn|SetItemName (Utilities|Struct|BreakS_Item _returnvalue)))))

(event EventMSGInteraction
  (params (Interaction :type E_Interaction%20Enum :default "NewEnumerator0") (Amount :type Integer) (FromActor :type Actor%20Object%20Reference) (Key :type Text))
  (bind _returnvalue (Actor|GetComponentbyClass FromActor "/Game/AntizeKitSystem/AntizeSystems/InventorySystem/Blueprints/BP_InventoryComponent.BP_InventoryComponent_C"))
  (bind _widget (Variables|Default|GetWidget))
  ;[1 1 1] Show/Hide Interact text
  (switch Utilities|FlowControl|Switch|SwitchonE_Interaction Interaction
    (:NewEnumerator0
      (Rendering|SetVisibility _widget true false)
      (CallFunction|RefreshInteract Key (Utilities|Struct|BreakS_InventorySlot (Variables|Setting|GetItemOnLoot))))
    (:NewEnumerator1
      (Rendering|SetVisibility _widget false false))
    (:NewEnumerator2
      ;;[1 1 1] If Loot is empty call destroy in ActorRef
      (if (> Amount 0)
        (Utilities|Struct|SetmembersinS_InventorySlot (Variables|Setting|GetItemOnLoot) Amount)
        (else
          (Utilities|IsValid _returnvalue
            (:Is%20Valid
              (Default|ServerDestroyActor _returnvalue self))))))))

(fn ConstructionScript
  (Utilities|FlowControl|Sequence
    (:then_0
      (CallFunction|MyNewConstruct))
    (:then_1
      ;[1 1 1] Set an unique ID
      (if (== (Variables|Setting|GetLootID) 0)
        (Variables|Setting|SetLootID (Math|Random|RandomInteger 999999999))))))

(fn DoSaveLoot
  (params (SaveRef :type BP%20Save%20Inventory%20Object%20Reference) (LootSavedID :type Array%20of%20Integers))
  (LocalVariables|SetLocal_Save SaveRef)
  (if (not (Variables|Setting|GetIgnoreSaving?))
    (LocalVariables|SetLocal_SaveLoot (Utilities|Struct|MakeS_SaveLoot (Variables|Setting|GetLootID) (Variables|Setting|GetItemOnLoot)))
    (bind _output_get (LocalVariables|SetLocal_FindIndex (Utilities|Array|FindItem LootSavedID (Variables|Setting|GetLootID))))
    (if (>= _output_get 0)
      (Utilities|Array|SetArrayElem (Variables|/Game/AntizeKitSystem/AntizeSystems/InventorySystem/Blueprints/SaveGame/BP_SaveInventory.BP_SaveInventory_C|GetSave_Loot (LocalVariables|GetLocal_Save)) (LocalVariables|GetLocal_FindIndex) (LocalVariables|GetLocal_SaveLoot) true)
      (else
        (Utilities|Array|Add (Variables|/Game/AntizeKitSystem/AntizeSystems/InventorySystem/Blueprints/SaveGame/BP_SaveInventory.BP_SaveInventory_C|GetSave_Loot (LocalVariables|GetLocal_Save)) (LocalVariables|GetLocal_SaveLoot))))
    (return)
    (else
      (return))))

(fn MyNewConstruct
  (bind _itemonloot (Variables|Setting|GetItemOnLoot))
  (bind _interactcorrection (Variables|Setting|GetInteractCorrection))
  (bind (_location _rotation _scale) (Utilities|Struct|BreakS_Correction _interactcorrection))
  ;[1 1 1] If item not found, get the first item
  (bind _returnvalue (Utilities|GetDataTableRow "/Game/AntizeKitSystem/AntizeSystems/InventorySystem/Logics/DT_Item.DT_Item" (.RowName (Utilities|Struct|BreakDataTableRowHandle (Utilities|Struct|BreakS_InventorySlot (Variables|Setting|GetItemOnLoot)))))
    (:then
      (LocalVariables|SetLocal_Item _returnvalue))
    (:RowNotFound
      (bind _outrownames (DataTable|GetDataTableRowNames "/Game/AntizeKitSystem/AntizeSystems/InventorySystem/Logics/DT_Item.DT_Item"))
      (Utilities|Struct|SetmembersinS_InventorySlot _itemonloot (Utilities|Struct|MakeDataTableRowHandle "/Game/AntizeKitSystem/AntizeSystems/InventorySystem/Logics/DT_Item.DT_Item" (Utilities|Array|Get(acopy) _outrownames)))))
  ;[1 1 1] Set minimum of amount to 1
  (if (> (Utilities|Struct|BreakS_InventorySlot _itemonloot) 0)
    _
    (else
      (Utilities|Struct|SetmembersinS_InventorySlot (Variables|Setting|GetItemOnLoot) 1)))
  (Components|StaticMesh|SetStaticMesh (Variables|Default|GetLoot_Mesh) (.PickupMesh (Utilities|Struct|BreakS_Item (LocalVariables|GetLocal_Item))))
  (Transformation|SetRelativeTransform (Variables|Default|GetLoot_Mesh) (Math|Transform|MakeTransform (.Location (Utilities|Struct|BreakS_Correction (.MeshCorrection (Utilities|Struct|BreakS_Item (LocalVariables|GetLocal_Item))))) (.Rotation (Utilities|Struct|BreakS_Correction (.MeshCorrection (Utilities|Struct|BreakS_Item (LocalVariables|GetLocal_Item))))) (.Scale (Utilities|Struct|BreakS_Correction (.MeshCorrection (Utilities|Struct|BreakS_Item (LocalVariables|GetLocal_Item)))))) false false)
  (Transformation|AddRelativeRotation (Variables|Default|GetArrow) (Variables|Setting|GetMeshRotCorrection) false false)
  (Transformation|SetRelativeTransform (Variables|Default|GetInteract) (Math|Transform|MakeTransform _location _rotation _scale) false false)
  (Transformation|SetRelativeLocation (Variables|Default|GetWidget) (Variables|Setting|GetPickUpTextLocCorrection) false false)
  (Rendering|Components|TextRender|SetText (Variables|Default|GetTextRender) (Utilities|Text|FormatText "({ItemName})" (.Name (Utilities|Struct|BreakS_Item (LocalVariables|GetLocal_Item)))))
  (bind _keys (Utilities|Map|Keys (.PickupMeshMaterial (Utilities|Struct|BreakS_Item (LocalVariables|GetLocal_Item)))))
  (if (> (Utilities|Array|Length _keys) 0)
    (for _array_element _keys
      (if (.ReturnValue (Utilities|Map|Find (.PickupMeshMaterial (Utilities|Struct|BreakS_Item (LocalVariables|GetLocal_Item))) _array_element))
        (Utilities|IsValid (.Value (Utilities|Map|Find (.PickupMeshMaterial (Utilities|Struct|BreakS_Item (LocalVariables|GetLocal_Item))) _array_element))
          (:Is%20Valid
            (Rendering|Material|SetMaterial (Variables|Default|GetLoot_Mesh) _array_element (.Value (Utilities|Map|Find (.PickupMeshMaterial (Utilities|Struct|BreakS_Item (LocalVariables|GetLocal_Item))) _array_element)))))))))

(fn OnRepItemonLoot
  ;[1 1 1] Unreal Engine 5 fix
  (CallFunction|MyNewConstruct)
  (return))

(fn MSGGetCamera
  (return 0))

(fn MSGGetDamageLocation
  (return "0, 0, 0"))

(fn MSGGetDestroyedLoot
  (return 0))

(fn MSGGetDropComponent
  (return 0))

(fn MSGGetInventory
  (return 0))

(fn MSGGetWeaponPlayerComponent
  (return 0 0))