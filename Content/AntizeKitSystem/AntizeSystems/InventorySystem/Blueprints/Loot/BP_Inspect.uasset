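; BP_Inspect is the 3D item preview actor for inspecting inventory items, rendered alone through a show-only SceneCapture2D.
; Construction applies the mesh, transform and per-slot material overrides from the item's examine data.
; Events drive timelines that spin the Base component on pitch or yaw, ease it to a target rotation, or zoom it by easing its relative location within a clamped radius.
; A Destroy event removes the actor.
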(event Custom|NewRotate
  (params (A :type Rotator) (B :type Rotator))
  ;[1 1 1] Set rotation
  (bind _value (Timeline|Timeline_Rotate PlayFromStart)
    (:Update
      (Transformation|SetRelativeRotation (Variables|Default|GetBase) (Math|Rotator|MakeRotator (Math|Rotator|NormalizeAxis (.roll (Math|Interpolation|Ease "Linear" _value A B true))) (Math|Rotator|NormalizeAxis (.pitch (Math|Interpolation|Ease "Linear" _value A B true))) (Math|Rotator|NormalizeAxis (.yaw (Math|Interpolation|Ease "Linear" _value A B true)))) false false))))

(event Custom|StopRotateY
  ;[1 1 1] Add rotate
  (bind _value (Timeline|Timeline_Y Stop)
    (:Update
      (Transformation|AddLocalRotation (Variables|Default|GetBase) (Math|Rotator|MakeRotator 0.0 (Math|Interpolation|Ease "Linear" _value (stale Custom|NewRotateY Speed) 0.0) 0.0) false false))))

(event Custom|NewRotateZ
  (params (Speed :type Float%20%28single-precision%29))
  ;[1 1 1] Add rotate
  (bind _value (Timeline|Timeline_Z PlayFromStart)
    (:Update
      (Transformation|AddLocalRotation (Variables|Default|GetBase) (Math|Rotator|MakeRotator 0.0 0.0 (Math|Interpolation|Ease "Linear" _value Speed 0.0)) false false))))

(event Custom|StopRotateZ
  ;[1 1 1] Add rotate
  (bind _value (Timeline|Timeline_Z Stop)
    (:Update
      (Transformation|AddLocalRotation (Variables|Default|GetBase) (Math|Rotator|MakeRotator 0.0 0.0 (Math|Interpolation|Ease "Linear" _value (stale Custom|NewRotateZ Speed) 0.0)) false false))))

(event Custom|Destroy
  ;[1 1 1] Destroy the actor
  (Actor|DestroyActor))

(event Custom|NewRotateY
  (params (Speed :type Float%20%28single-precision%29))
  ;[1 1 1] Add rotate
  (bind _value (Timeline|Timeline_Y PlayFromStart)
    (:Update
      (Transformation|AddLocalRotation (Variables|Default|GetBase) (Math|Rotator|MakeRotator 0.0 (Math|Interpolation|Ease "Linear" _value Speed 0.0) 0.0) false false))))

(event Custom|OnZoom
  (params (A :type Vector) (B :type Vector))
  ;[1 1 1] Zoom In/Out
  (bind _value (Timeline|Timeline_Zoom PlayFromStart)
    (:Update
      (Transformation|SetRelativeLocation (Variables|Default|GetBase) (Math|Vector|ClampVectorSize (Math|Interpolation|Ease "Linear" _value A B) 0.0 25.0) false false))))

(fn ConstructionScript
  (CallFunction|MyNewConstruct))

(fn MyNewConstruct
  (bind _itemdata (Variables|Spawn|GetItemData))
  (bind _itemdata_2 (Variables|Spawn|GetItemData))
  (bind _examinedata (Utilities|Struct|BreakS_Item _itemdata))
  (bind _examinedata_2 (Utilities|Struct|BreakS_Item _itemdata_2))
  (bind (_3ditemmesh _3ditemtransform) (Utilities|Struct|BreakS_Examine _examinedata))
  (bind _3ditemmeshmaterial (Utilities|Struct|BreakS_Examine _examinedata_2))
  (Rendering|SceneCapture|ShowOnlyActorComponents (Variables|Default|GetSceneCaptureComponent2D) self)
  (Components|StaticMesh|SetStaticMesh (Variables|Default|GetItemMesh) _3ditemmesh)
  (Transformation|SetRelativeTransform (Variables|Default|GetItemMesh) _3ditemtransform false false)
  (bind _keys (Utilities|Map|Keys _3ditemmeshmaterial))
  (if (> (Utilities|Array|Length _keys) 0)
    (for _array_element _keys
      (if (.ReturnValue (Utilities|Map|Find _3ditemmeshmaterial _array_element))
        (Utilities|IsValid (.Value (Utilities|Map|Find _3ditemmeshmaterial _array_element))
          (:Is%20Valid
            (Rendering|Material|SetMaterial (Variables|Default|GetItemMesh) _array_element (.Value (Utilities|Map|Find _3ditemmeshmaterial _array_element)))))))))