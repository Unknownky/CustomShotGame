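; Blueprint interface for the AntizeKit inventory system, declaring messages that other objects implement to talk to it.
; Calls cover interactions with amount, source actor and key, tracking of destroyed loot IDs, sound playback at a location, and damage display.
; Getters expose the inventory, drop component, weapon player component, camera, and damage location.
; All functions are empty declarations, so behavior lives entirely in the implementers.
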(fn MSGInteraction
  (params (Interaction :type E_Interaction%20Enum :default "NewEnumerator0") (Amount :type Integer) (FromActor :type Actor%20Object%20Reference) (Key :type Text)))

(fn MSGAddDestroyedLoot
  (params (LootID :type Integer)))

(fn MSGGetDestroyedLoot
  (return 0))

(fn MSGPlaySoundatLocation
  (params (Sound :type Sound%20Cue%20Object%20Reference) (Location :type Vector)))

(fn MSGGetInventory
  (return 0))

(fn MSGGetDropComponent
  (return 0))

(fn MSGShowDamage
  (params (Location :type Vector) (Damage :type Float%20%28single-precision%29)))

(fn MSGGetDamageLocation
  (return "0, 0, 0"))

(fn MSGGetWeaponPlayerComponent
  (return 0 0))

(fn MSGGetCamera
  (return 0))