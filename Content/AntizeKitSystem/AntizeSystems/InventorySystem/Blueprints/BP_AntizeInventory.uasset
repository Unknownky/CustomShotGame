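; Shared helper functions for the Antize inventory system, covering save games, world loot persistence and slot UI.
; Save helpers load or create BP_SaveInventory and stamp each save with a count and date.
; Loot helpers match BP_Loot actors to saved IDs, destroying depleted ones, while a validator prints warnings for duplicate storage, loot and door identifiers.
; UI helpers reset slot styles, map values to red-to-green colors and test directional keys.
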(fn ResetSyleonSlot
  (params (Object :type Widget%20Object%20Reference))
  (bind _asw_inventory_slot (Utilities|Casting|CastToW_InventorySlot Object)
    (:then
      (Default|ResetInventorySlotStyle _asw_inventory_slot))
    (:CastFailed
      (bind _asw_storage_slot (Utilities|Casting|CastToW_StorageSlot Object)
        (:then
          (Default|ResetStorageSlotStyle _asw_storage_slot false))
        (:CastFailed
          (return)))))
  (return))

(fn MyLoadGame
  (params (SlotName :type String) (UserIndex :type Integer))
  ;[1 1 1] Get slot
  (LocalVariables|SetLocal_SlotName SlotName)
  (LocalVariables|SetLocal_UserIndex UserIndex)
  ;[1 1 1] Check if save exist
  (bind _returnvalue (SaveGame|DoesSaveGameExist (LocalVariables|GetLocal_SlotName) (LocalVariables|GetLocal_UserIndex)))
  (if _returnvalue
    ;[1 1 1] Load save
    (bind _returnvalue_2 (SaveGame|LoadGamefromSlot (LocalVariables|GetLocal_SlotName) (LocalVariables|GetLocal_UserIndex)))
    (bind _asbp_save_inventory (Utilities|Casting|CastToBP_SaveInventory _returnvalue_2)
      (:then
        (return _asbp_save_inventory))
      (:CastFailed
        (return 0)))
    (else
      ;[1 1 1] Create new save
      (bind _returnvalue_3 (SaveGame|CreateSaveGameObject "/Game/AntizeKitSystem/AntizeSystems/InventorySystem/Blueprints/SaveGame/BP_SaveInventory.BP_SaveInventory_C"))
      (return _returnvalue_3))))

(fn MySaveGame
  (params (SaveGameObject :type BP%20Save%20Inventory%20Object%20Reference))
  ;[1 1 1] Get slot
  (bind _output_get (LocalVariables|SetLocal_SlotsSave SaveGameObject))
  (Math|Integer|IncrementInt (Variables|/Game/AntizeKitSystem/AntizeSystems/InventorySystem/Blueprints/SaveGame/BP_SaveInventory.BP_SaveInventory_C|GetNumberSave _output_get)
    (:%20%20
      (Variables|/Game/AntizeKitSystem/AntizeSystems/InventorySystem/Blueprints/SaveGame/BP_SaveInventory.BP_SaveInventory_C|SetDateSaved (LocalVariables|GetLocal_SlotsSave) (Math|DateTime|Now))
      ;[1 1 1] Perfom save
      (bind _returnvalue (SaveGame|SaveGametoSlot (LocalVariables|GetLocal_SlotsSave) (Variables|/Game/AntizeKitSystem/AntizeSystems/InventorySystem/Blueprints/SaveGame/BP_SaveInventory.BP_SaveInventory_C|GetSlotName (LocalVariables|GetLocal_SlotsSave))))
      (return _returnvalue))))

(fn GetColorbyValue
  (params (Value :type Float%20%28single-precision%29))
  (return (select (<= Value 0.1) "(R=1.000000,G=0.000000,B=0.000000,A=1.000000)" (select (<= Value 0.3) "(R=1.000000,G=0.058824,B=0.000000,A=1.000000)" (select (<= Value 0.5) "(R=1.000000,G=0.345098,B=0.000000,A=1.000000)" (select (<= Value 0.6) "(R=0.992157,G=1.000000,B=0.003922,A=1.000000)" (select (<= Value 0.95) "(R=0.674510,G=1.000000,B=0.000000,A=1.000000)" "(R=0.050980,G=1.000000,B=0.000000,A=1.000000)")))))))

(fn GetSlotNameUserIndex
  (return "MySaveName" 0))

(fn GetIsDirectionKey
  (params (Direction :type E_Pad%20Enum :default "NewEnumerator0") (Key :type Key%20Structure))
  (LocalVariables|SetLocal_Key Key)
  (return (Utilities|Select :Index Direction :NewEnumerator0 (Math|Boolean|ORBoolean (== (LocalVariables|GetLocal_Key) "Gamepad_LeftStick_Up") (== (LocalVariables|GetLocal_Key) "Gamepad_DPad_Up") (== (LocalVariables|GetLocal_Key) "Up")) :NewEnumerator1 (Math|Boolean|ORBoolean (== (LocalVariables|GetLocal_Key) "Gamepad_LeftStick_Down") (== (LocalVariables|GetLocal_Key) "Gamepad_DPad_Down") (== (LocalVariables|GetLocal_Key) "Down")) :NewEnumerator2 (Math|Boolean|ORBoolean (== (LocalVariables|GetLocal_Key) "Gamepad_LeftStick_Left") (== (LocalVariables|GetLocal_Key) "Gamepad_DPad_Left") (== (LocalVariables|GetLocal_Key) "Left")) :NewEnumerator3 (Math|Boolean|ORBoolean (== (LocalVariables|GetLocal_Key) "Gamepad_RightStick_Right") (== (LocalVariables|GetLocal_Key) "Gamepad_DPad_Right") (== (LocalVariables|GetLocal_Key) "Right")) :NewEnumerator4 false)))

(fn ApplyLootWorld
  ;[1 1 1] If loot can be modified by saving, apply loaded data
  (bind _saveref (Class|BPAntizeKitInterface|MSGGetSave(Message) (Game|GetGameInstance)))
  (bind _output_get (LocalVariables|SetLocal_Save _saveref))
  (Utilities|IsValid _output_get
    (:Is%20Valid
      (bind _local_lootid (InventorySystem|Save/Load|GetLootSavedID _output_get))
      (LocalVariables|SetLocal_LootID _local_lootid)
      (if (> (Utilities|Array|Length (LocalVariables|GetLocal_LootID)) 0)
        (bind _outactors (Actor|GetAllActorsOfClass 0 "/Game/AntizeKitSystem/AntizeSystems/InventorySystem/Blueprints/Loot/BP_Loot.BP_Loot_C"))
        (for _array_element _outactors
          (if (not (Variables|/Game/AntizeKitSystem/AntizeSystems/InventorySystem/Blueprints/Loot/BP_Loot.BP_Loot_C|GetIgnoreSaving? _array_element))
            (bind _output_get_2 (LocalVariables|SetLocal_FindIndex (Utilities|Array|FindItem (LocalVariables|GetLocal_LootID) (Variables|/Game/AntizeKitSystem/AntizeSystems/InventorySystem/Blueprints/Loot/BP_Loot.BP_Loot_C|GetLootID _array_element))))
            (if (>= _output_get_2 0)
              (if (<= (Utilities|Struct|BreakS_InventorySlot (Utilities|Struct|BreakS_SaveLoot (Utilities|Array|Get(acopy) (Variables|/Game/AntizeKitSystem/AntizeSystems/InventorySystem/Blueprints/SaveGame/BP_SaveInventory.BP_SaveInventory_C|GetSave_Loot (LocalVariables|GetLocal_Save)) (LocalVariables|GetLocal_FindIndex)))) 0)
                (Actor|DestroyActor _array_element)
                (else
                  (Variables|/Game/AntizeKitSystem/AntizeSystems/InventorySystem/Blueprints/Loot/BP_Loot.BP_Loot_C|SetItemOnLoot _array_element ""))))))
        (return)
        (else
          (return))))
    (:Is%20Not%20Valid
      (return))))

(fn CheckforDuplicateName
  (bind _local_doorname (LocalVariables|GetLocal_DoorName))
  (bind _local_lootid (LocalVariables|GetLocal_LootID))
  ;[1 1 1] Print a warning message if duplicated save setting or name is found
  (bind _outactors (Actor|GetAllActorsOfClass 0 "/Game/AntizeKitSystem/AntizeSystems/InventorySystem/Blueprints/Storage/BP_MasterStorage.BP_MasterStorage_C"))
  (for _array_element _outactors
    (if (Utilities|Enum|NotEqual(Enum) (Variables|/Game/AntizeKitSystem/AntizeSystems/InventorySystem/Blueprints/Storage/BP_MasterStorage.BP_MasterStorage_C|GetStorageName _array_element) "NewEnumerator0")
      (if (Utilities|Array|ContainsItem (LocalVariables|GetLocal_Name) (Variables|/Game/AntizeKitSystem/AntizeSystems/InventorySystem/Blueprints/Storage/BP_MasterStorage.BP_MasterStorage_C|GetStorageName _array_element))
        (Development|PrintString 0 (Utilities|String|Append "Warning : Duplicate Storage Name - " (Utilities|String|EnumtoString (Variables|/Game/AntizeKitSystem/AntizeSystems/InventorySystem/Blueprints/Storage/BP_MasterStorage.BP_MasterStorage_C|GetStorageName _array_element)) " -> " (Utilities|GetDisplayName _array_element) " (E_SaveName)") true true "(R=1.000000,G=0.677696,B=0.000000,A=1.000000)" 1e+01)
        (else
          (Utilities|Array|Add (LocalVariables|GetLocal_Name) (Variables|/Game/AntizeKitSystem/AntizeSystems/InventorySystem/Blueprints/Storage/BP_MasterStorage.BP_MasterStorage_C|GetStorageName _array_element))))))
  (bind _outactors_2 (Actor|GetAllActorsOfClass 0 "/Game/AntizeKitSystem/AntizeSystems/InventorySystem/Blueprints/Loot/BP_Loot.BP_Loot_C"))
  (for _array_element_2 _outactors_2
    (if (Utilities|Array|ContainsItem _local_lootid (Variables|/Game/AntizeKitSystem/AntizeSystems/InventorySystem/Blueprints/Loot/BP_Loot.BP_Loot_C|GetLootID _array_element_2))
      (Development|PrintString 0 (Utilities|String|Append "Warning : Duplicate Loot ID " " -> " (Utilities|String|ToString(Integer) (Variables|/Game/AntizeKitSystem/AntizeSystems/InventorySystem/Blueprints/Loot/BP_Loot.BP_Loot_C|GetLootID _array_element_2)) " -> " (Utilities|GetDisplayName _array_element_2)) true true "(R=1.000000,G=0.677696,B=0.000000,A=1.000000)" 1e+01)
      (else
        (Utilities|Array|Add _local_lootid (Variables|/Game/AntizeKitSystem/AntizeSystems/InventorySystem/Blueprints/Loot/BP_Loot.BP_Loot_C|GetLootID _array_element_2)))))
  (bind _outactors_3 (Actor|GetAllActorsOfClass 0 "/Game/AntizeKitSystem/AntizeSystems/InventorySystem/Blueprints/Demo/BP_Door.BP_Door_C"))
  (for _array_element_3 _outactors_3
    (if (Utilities|Array|ContainsItem _local_doorname (Utilities|GetDisplayName _array_element_3))
      (Development|PrintString 0 (Utilities|String|Append "Warning : Duplicate Door Name - " " -> " (Utilities|GetDisplayName _array_element_3)) true true "(R=1.000000,G=0.677696,B=0.000000,A=1.000000)" 1e+01)
      (else
        (Utilities|Array|Add _local_doorname (Utilities|GetDisplayName _array_element_3)))))
  (return))

(fn GetLootSavedID
  (params (SaveRef :type BP%20Save%20Inventory%20Object%20Reference))
  (if (Variables|/Game/AntizeKitSystem/AntizeSystems/InventorySystem/Blueprints/SaveGame/BP_SaveInventory.BP_SaveInventory_C|GetSaved? SaveRef)
    (bind _output_get (LocalVariables|SetLocal_Save SaveRef))
    (for _array_element (Variables|/Game/AntizeKitSystem/AntizeSystems/InventorySystem/Blueprints/SaveGame/BP_SaveInventory.BP_SaveInventory_C|GetSave_Loot _output_get)
      (Utilities|Array|Add (LocalVariables|GetLocal_Loot_ID) (Utilities|Struct|BreakS_SaveLoot _array_element)))
    (return (LocalVariables|GetLocal_Loot_ID))
    (else
      (return (LocalVariables|GetLocal_Loot_ID)))))

(fn AddDestroyedLoot
  (params (InLootDestroyed :type Array%20of%20Integers) (LootID :type Integer%20%28by%20ref%29))
  ;[1 1 1] Add loot in destroyed array
  (if (Utilities|Array|ContainsItem InLootDestroyed LootID)
    _
    (else
      (Utilities|Array|Add InLootDestroyed LootID)))
  (return InLootDestroyed))