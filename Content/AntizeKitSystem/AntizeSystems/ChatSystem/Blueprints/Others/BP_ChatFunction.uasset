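; BP_ChatFunction is a chat system helper that provides a time-of-day text and broadcasts system messages to players.
; GetActualTime formats the current hour and minute from Now as HH:MM text.
; SendSystemMessageToPlayers loops over the valid entries in a connected-player list and sends each a new-message interface call.
; That message is marked received and carries the text under a fixed category, with sender and recipient IDs set to -1.
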(fn GetActualTime
  (bind _returnvalue (Math|DateTime|Now))
  (bind _returnvalue_2 (TimeOfDay|GetTimeOfDay _returnvalue :!class /Script/Engine.KismetMathLibrary))
  (return (Utilities|Text|FormatText "{HH}:{MM}" (Utilities|Text|ToText(Integer) (.hours _returnvalue_2) false true 2 2) (Utilities|Text|ToText(Integer) (.minutes _returnvalue_2) false true 2 2))))

(fn SendSystemMessagetoPlayers
  (params (ConnectedPlayers :type Array%20of%20Controller%20Object%20References) (Message :type Text))
  ;[1 1 1] Sends a system message to players
  (for _array_element ConnectedPlayers
    (Utilities|IsValid _array_element
      (:Is%20Valid
        (Class|BPAntizeChatInterface|MSGNewMessage(Message) _array_element true (Utilities|Struct|MakeS_MessageData "NewEnumerator5" -1 -1 Message)))))
  (return))