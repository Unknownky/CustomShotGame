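; Base door remote that unlocks its linked doors when a player interacts with it.
; On BeginPlay it registers itself in each linked door's remote list, and it toggles an interact widget by radius.
; Interaction runs on the server: if active, it unlocks the doors, and either way it multicasts a success or error sound.
; An overridable SetIsLockedRemote copies IsLocked into IsActive and swaps the red or green emissive material.
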(event Custom|Multi_PlaySoundAtLocation
  (params (Sound :type Sound%20Cue%20Object%20Reference))
  ;[1 1 1] Play sound at location (From Server->Multi)
  (Audio|PlaySoundatLocation Sound (Transformation|GetActorLocation)))

(event Custom|OnServer_OnInteract
  ;[1 1 1] Interact if the remote is active else play a sound
  (Networking|SwitchHasAuthority
    (:Authority
      (if (Variables|Default|GetIsActive?)
        (for _array_element (Variables|Settings|GetLinkedDoorRef)
          (Utilities|IsValid _array_element
            (:Is%20Valid
              (Default|OnServerSetIsLockedDoor _array_element false false))))
        (CallFunction|MultiPlaySoundatLocation "/Game/AntizeKitSystem/AntizeSystems/DoorSystem/Ressources/Audio/Cue_CardCorrect.Cue_CardCorrect")
        (else
          (CallFunction|MultiPlaySoundatLocation "/Game/AntizeKitSystem/AntizeSystems/DoorSystem/Ressources/Audio/Cue_Error.Cue_Error"))))))

(event EventBeginPlay
  ;[1 1 1] Constructeur
  (for _array_element (Variables|Settings|GetLinkedDoorRef)
    (Utilities|IsValid _array_element
      (:Is%20Valid
        (Utilities|Array|Add (Variables|/Game/AntizeKitSystem/AntizeSystems/DoorSystem/Blueprints/Door/BP_MasterDoor.BP_MasterDoor_C|GetLinkedRemote _array_element) self)))))

(fn ConstructionScript)

(fn UpdateInteraction
  (params (Interaction :type E_Interaction%20Enum :default "NewEnumerator0"))
  (bind _w_interact (Variables|Default|GetW_Interact))
  ;[1 1 1] Show/Hide Interact button
  (switch Utilities|FlowControl|Switch|SwitchonE_Interaction Interaction
    (:NewEnumerator0
      (Rendering|SetVisibility _w_interact true false))
    (:NewEnumerator1
      (Rendering|SetVisibility _w_interact false false))
    (:NewEnumerator2
      (return)))
  (return))

(fn SetIsLockedRemote
  (params (IsLocked? :type Boolean))
  ;[1 1 1] Don't forget, can be overrided on children to make your code (Multicast)
  (Variables|Default|SetIsActive? IsLocked?)
  (Rendering|Material|SetMaterial (Variables|Default|GetSM_Remote) 2 (select IsLocked? "/Game/AntizeKitSystem/AntizeSystems/DoorSystem/Ressources/Materials/MI_Emissive_Red.MI_Emissive_Red" "/Game/AntizeKitSystem/AntizeSystems/DoorSystem/Ressources/Materials/MI_Emissive_Green.MI_Emissive_Green"))
  (return))