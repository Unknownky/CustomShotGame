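; Base networked keypad actor that unlocks its linked doors when the correct code is entered on its widget.
; BeginPlay registers the keypad with each door and binds the widget; the server checks codes, counts attempts and can lock out all keypads on shared doors.
; Multicasts update widget, indicator material and sounds through child-overridable functions.
; Lock-state updates pass through a DoOnce with retriggerable delay to filter repeated calls.
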(event Custom|Multi_RefreshWidget
  (params (CurrentText :type String))
  ;[1 1 1] Refresh Widget (From server->Multi)
  (Rendering|Components|TextRender|SetText (Variables|/Game/AntizeKitSystem/AntizeSystems/DoorSystem/Widgets/W_KeyPad.W_KeyPad_C|GetTextBlock_CurrentCode (Variables|Spawn|GetW_KeyPadRef)) (Utilities|Text|ToText(String) CurrentText)))

(event Custom|Multi_OnIncorrectCode
  ;[1 1 1] Call OnIncorrectCode (From server->Multi)
  (CallFunction|OnMultionIncorrectCode)
  (Default|OnMultionIncorrectCode (Variables|Spawn|GetW_KeyPadRef)))

(event Custom|Multi_PlaySound
  (params (Sound :type Sound%20Cue%20Object%20Reference))
  ;[1 1 1] Play sound at location (From Server->Multi)
  (Audio|PlaySoundatLocation Sound (Transformation|GetActorLocation)))

(event Custom|Multi_OnMaxAttempt
  ;[1 1 1] Call OnMaxAttempt (From server->Multi)
  (CallFunction|OnMultionMaxAttempt)
  (Default|OnMultionMaxAttempt (Variables|Spawn|GetW_KeyPadRef)))

(event Custom|ShowDebug
  ;[1 1 1] Show debug
  (if (Variables|Spawn|GetDebug?) :!label _label
    (Utilities|FlowControl|Delay 0.2)
    (Development|PrintString (Utilities|String|ToString(Boolean) (Variables|Default|GetIsError?)))
    (goto _label)))

(event Custom|CallSetIsLockedKeyPad
  (params (IsLocked? :type Boolean) (IsLoading? :type Boolean))
  ;[1 1 1] Call only once SetIsLockedKeyPad
  (Utilities|FlowControl|DoOnce false :!label _label
    (:Completed
      (CallFunction|OnMultiSetIsLockedKeyPad IsLocked? IsLoading?)
      (Utilities|FlowControl|RetriggerableDelay 0.2)
      (goto _label Reset))))

(event EventBeginPlay
  ;[1 1 1] Constructeur
  (for _array_element (Variables|Settings|GetLinkedDoorRef)
    (Utilities|IsValid _array_element
      (:Is%20Valid
        (Utilities|Array|Add (Variables|/Game/AntizeKitSystem/AntizeSystems/DoorSystem/Blueprints/Door/BP_MasterDoor.BP_MasterDoor_C|GetLinkedKeyPad _array_element) self))))
  (bind _asw_key_pad (Utilities|Casting|CastToW_KeyPad (UserInterface|GetUserWidgetObject (Variables|Default|GetW_KeyPad))))
  (Variables|Spawn|SetW_KeyPadRef _asw_key_pad)
  (Variables|/Game/AntizeKitSystem/AntizeSystems/DoorSystem/Widgets/W_KeyPad.W_KeyPad_C|SetKeyPadRef (Variables|Spawn|GetW_KeyPadRef) self)
  ;[1 1 1] Show debug
  (CallFunction|ShowDebug))

(fn ConstructionScript)

(fn OnServerCheckCode
  (params (Code :type String))
  (bind _actualattempt (Variables|Settings|Attempt|GetActualAttempt))
  (Networking|SwitchHasAuthority
    (:Authority
      (if (Utilities|Enum|Equal(Enum) Code (Variables|Settings|GetCode))
        ;[1 1 1] On correct code -> Unlock all doors linked and change the indicator
        (for _array_element (Variables|Settings|GetLinkedDoorRef)
          (Utilities|IsValid _array_element
            (:Is%20Valid
              (Default|OnServerSetIsLockedDoor _array_element false false))))
        (return)
        (else
          ;[1 1 1] On incorrect code
          (if (> (Variables|Settings|Attempt|GetMaxAttempt) 0)
            (Math|Integer|IncrementInt _actualattempt
              (:%20%20
                (if (>= _actualattempt (Variables|Settings|Attempt|GetMaxAttempt))
                  (Variables|Default|SetIsError? true)
                  (if (Variables|Settings|Attempt|GetDisableAllKeypads?)
                    ;[1 1 1] Disable all keypad
                    (for _array_element_2 (Variables|Settings|GetLinkedDoorRef)
                      (Utilities|IsValid _array_element_2
                        (:Is%20Valid
                          (for _array_element_3 (Variables|/Game/AntizeKitSystem/AntizeSystems/DoorSystem/Blueprints/Door/BP_MasterDoor.BP_MasterDoor_C|GetLinkedKeyPad _array_element_2)
                            (Utilities|IsValid _array_element_3
                              (:Is%20Valid
                                (bind _returnvalue (Utilities|Array|AddUnique (LocalVariables|GetLocal_AlreadyDo) _array_element_3))
                                (if (>= _returnvalue 0)
                                  (CallFunction|MultionMaxAttempt _array_element_3))))))))
                    (return)
                    (else
                      (CallFunction|MultionMaxAttempt)))
                  (else
                    (CallFunction|MultionIncorrectCode :!label _label)))))
            (else
              (goto _label)))
          (return))))))

(fn OnMultionIncorrectCode
  ;[1 1 1] Can be overrided on children to make your code (Multicast)
  (Audio|PlaySoundatLocation "/Game/AntizeKitSystem/AntizeSystems/DoorSystem/Ressources/Audio/Cue_IncorrectCode.Cue_IncorrectCode" (Transformation|GetActorLocation))
  (return))

(fn OnMultiSetIsLockedKeyPad
  (params (IsLocked? :type Boolean) (IsLoading :type Boolean))
  ;[1 1 1] Don't forget, can be overrided on children to make your code (Multicast)
  (LocalVariables|SetLocal_IsLoading? IsLoading)
  (if (not (Variables|Default|GetIsError?))
    (Rendering|Material|SetMaterial (Variables|Default|GetSM_KeyPad) 2 (select IsLocked? "/Game/AntizeKitSystem/AntizeSystems/DoorSystem/Ressources/Materials/MI_Emissive_Red.MI_Emissive_Red" "/Game/AntizeKitSystem/AntizeSystems/DoorSystem/Ressources/Materials/MI_Emissive_Green.MI_Emissive_Green"))
    (if (not IsLocked?)
      (Default|OnMultionCorrectCode (Variables|Spawn|GetW_KeyPadRef))
      (if (not (LocalVariables|GetLocal_IsLoading?))
        (Audio|PlaySoundatLocation "/Game/AntizeKitSystem/AntizeSystems/DoorSystem/Ressources/Audio/Cue_CorrectCode.Cue_CorrectCode" (Transformation|GetActorLocation))
        (return)
        (else
          (return)))
      (else
        (return)))
    (else
      (Default|OnMultionMaxAttempt (Variables|Spawn|GetW_KeyPadRef))
      (CallFunction|OnMultionMaxAttempt)
      (return))))

(fn OnMultionMaxAttempt
  ;[1 1 1] Can be overrided on children to make your code (Multicast)
  (Rendering|Material|SetMaterial (Variables|Default|GetSM_KeyPad) 2 "/Game/AntizeKitSystem/AntizeSystems/DoorSystem/Ressources/Materials/MI_Emissive_Yellow.MI_Emissive_Yellow")
  (Audio|PlaySoundatLocation "/Game/AntizeKitSystem/AntizeSystems/DoorSystem/Ressources/Audio/Cue_CardWrong.Cue_CardWrong" (Transformation|GetActorLocation))
  (return))