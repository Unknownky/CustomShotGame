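; BP_DoorSystem saves and restores the locked state of every BP_MasterDoor in the world, keyed by DoorID.
; GetDoorWorld merges current lock states into saved entries, and SaveDoorData writes the given array to a single BP_DoorSave slot.
; ApplyDoorWorld reapplies saved locks through each door's OnServerSetIsLockedDoor and warns about duplicate IDs.
; A separate helper parses a number from the end of the engine version string.
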(fn SaveDoorData
  (params (DoorSaved :type Array%20of%20S%20Door%20Saved%20Structures))
  ;[1 1 1] Get/Create save and set variable
  (LocalVariables|SetLocal_DoorSaved DoorSaved)
  (bind _returnvalue (SaveGame|DoesSaveGameExist "Door\\DoorSaved"))
  (if _returnvalue
    (bind _returnvalue_2 (SaveGame|LoadGamefromSlot "Door\\DoorSaved"))
    (bind _asbp_door_save (Utilities|Casting|CastToBP_DoorSave _returnvalue_2)
      (:then
        (LocalVariables|SetLocal_Save _asbp_door_save))
      (:CastFailed
        (Development|PrintString 0 "BP_DoorSystem->SaveDoorData->BP_DoorSave is not valid (Maybe you changed the save bp)" true true "(R=1.000000,G=0.170426,B=0.030634,A=1.000000)" 1e+01)
        (bind _returnvalue_3 (SaveGame|CreateSaveGameObject "/Game/AntizeKitSystem/AntizeSystems/DoorSystem/Blueprints/Save/BP_DoorSave.BP_DoorSave_C" :!label _label))
        (LocalVariables|SetLocal_Save _returnvalue_3)))
    (else
      (goto _label)))
  (Variables|/Game/AntizeKitSystem/AntizeSystems/DoorSystem/Blueprints/Save/BP_DoorSave.BP_DoorSave_C|SetDoorSaved (LocalVariables|GetLocal_Save) (LocalVariables|GetLocal_DoorSaved))
  ;[1 1 1] Perfom save
  (bind _returnvalue_4 (SaveGame|SaveGametoSlot (LocalVariables|GetLocal_Save) "Door\\DoorSaved"))
  (return _returnvalue_4))

(fn LoadDoorData
  ;[1 1 1] Check if save exist
  (bind _returnvalue (SaveGame|DoesSaveGameExist "Door\\DoorSaved"))
  (if _returnvalue
    ;[1 1 1] Load save (Change SaveIndex by level)
    (bind _returnvalue_2 (SaveGame|LoadGamefromSlot "Door\\DoorSaved"))
    (bind _asbp_door_save (Utilities|Casting|CastToBP_DoorSave _returnvalue_2)
      (:then
        (return (Variables|/Game/AntizeKitSystem/AntizeSystems/DoorSystem/Blueprints/Save/BP_DoorSave.BP_DoorSave_C|GetDoorSaved _asbp_door_save)))
      (:CastFailed
        (Development|PrintString 0 "BP_DoorSystem->LoadDoorData->BP_DoorSave is not valid (Maybe you changed the save bp)" true true "(R=1.000000,G=0.170426,B=0.030634,A=1.000000)" 1e+01)
        (return (Utilities|Array|MakeArray))))
    (else
      (return (Utilities|Array|MakeArray)))))

(fn ApplyDoorWorld
  (bind (_door_id _doorsaved) (DoorSystem|GetDoorSavedID))
  (LocalVariables|SetLocal_Door_ID _door_id)
  (LocalVariables|SetLocal_DoorSaved _doorsaved)
  (bind _outactors (Actor|GetAllActorsOfClass 0 "/Game/AntizeKitSystem/AntizeSystems/DoorSystem/Blueprints/Door/BP_MasterDoor.BP_MasterDoor_C"))
  (for _array_element _outactors
    (Utilities|IsValid _array_element
      (:Is%20Valid
        (LocalVariables|SetLocal_ActualID (Variables|/Game/AntizeKitSystem/AntizeSystems/DoorSystem/Blueprints/Door/BP_MasterDoor.BP_MasterDoor_C|GetDoor_ID _array_element))
        (if (< (Utilities|Array|FindItem (LocalVariables|GetLocal_UniqueID) (LocalVariables|GetLocal_ActualID)) 0)
          (Utilities|Array|Add (LocalVariables|GetLocal_UniqueID) (LocalVariables|GetLocal_ActualID))
          (else
            (Development|PrintString 0 (Utilities|String|Append "Warning : Door ID '" (Utilities|String|ToString(Integer) (LocalVariables|GetLocal_ActualID)) "' already exists, please refresh the door ID of  " (Utilities|GetDisplayName _array_element)) true true "(R=1.000000,G=0.285550,B=0.000000,A=1.000000)" 25.0)))
        (bind _output_get (LocalVariables|SetLocal_FindIndex (Utilities|Array|FindItem (LocalVariables|GetLocal_Door_ID) (LocalVariables|GetLocal_ActualID))))
        (if (>= _output_get 0)
          (Default|OnServerSetIsLockedDoor _array_element (Utilities|Struct|BreakS_DoorSaved (Utilities|Array|Get(acopy) (LocalVariables|GetLocal_DoorSaved) (LocalVariables|GetLocal_FindIndex))) true)))))
  (return))

(fn GetDoorWorld
  (bind (_door_id _doorsaved) (DoorSystem|GetDoorSavedID))
  (LocalVariables|SetLocal_Door_ID _door_id)
  (LocalVariables|SetLocal_DoorSaved _doorsaved)
  (bind _outactors (Actor|GetAllActorsOfClass 0 "/Game/AntizeKitSystem/AntizeSystems/DoorSystem/Blueprints/Door/BP_MasterDoor.BP_MasterDoor_C"))
  (for _array_element _outactors
    (Utilities|IsValid _array_element
      (:Is%20Valid
        (bind _output_get (LocalVariables|SetLocal_FindIndex (Utilities|Array|FindItem (LocalVariables|GetLocal_Door_ID) (Variables|/Game/AntizeKitSystem/AntizeSystems/DoorSystem/Blueprints/Door/BP_MasterDoor.BP_MasterDoor_C|GetDoor_ID _array_element))))
        (LocalVariables|SetLocal_DoorData (Utilities|Struct|MakeS_DoorSaved (Variables|/Game/AntizeKitSystem/AntizeSystems/DoorSystem/Blueprints/Door/BP_MasterDoor.BP_MasterDoor_C|GetDoor_ID _array_element) (Default|GetIsDoorLocked _array_element)))
        (if (>= _output_get 0)
          (Utilities|Array|SetArrayElem (LocalVariables|GetLocal_DoorSaved) (LocalVariables|GetLocal_FindIndex) (LocalVariables|GetLocal_DoorData))
          (else
            (Utilities|Array|Add (LocalVariables|GetLocal_DoorSaved) (LocalVariables|GetLocal_DoorData)))))))
  (return (LocalVariables|GetLocal_DoorSaved)))

(fn GetDoorSavedID
  (bind _doorsaved (DoorSystem|LoadDoorData))
  (bind _output_get (LocalVariables|SetLocal_DoorSaved _doorsaved))
  (if (> (Utilities|Array|Length _output_get) 0)
    (for _array_element (LocalVariables|GetLocal_DoorSaved)
      (Utilities|Array|Add (LocalVariables|GetLocal_Door_ID) (Utilities|Struct|BreakS_DoorSaved _array_element))))
  (return (LocalVariables|GetLocal_Door_ID) (LocalVariables|GetLocal_DoorSaved)))

(fn MyGetEngineVersion
  (bind _returnvalue (Development|GetEngineVersion))
  (bind _index (Utilities|FlowControl|ForLoopwithBreak 1 6 :!label _label)
    (:LoopBody
      (LocalVariables|SetLocal_Index _index)
      (bind _output_get (LocalVariables|SetLocal_Substring (Utilities|String|GetSubstring _returnvalue (- (Utilities|String|Len _returnvalue) (- 6 (LocalVariables|GetLocal_Index))) (- 6 (LocalVariables|GetLocal_Index)))))
      (if (> (Math|Conversions|ToInteger(Byte) _output_get) 0)
        (LocalVariables|SetLocal_Version (Math|Conversions|ToInteger(Byte) (LocalVariables|GetLocal_Substring)))
        (goto _label Break)))
    (:Completed
      (return (LocalVariables|GetLocal_Version)))))