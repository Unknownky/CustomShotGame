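; Player pawn component that handles interaction with doors, remote actors and widget keypads in the door system.
; On the locally controlled pawn, a timer-driven camera line trace tracks the actor in sight, and interacting opens, closes, locks or unlocks doors or triggers remotes.
; It relays actions, sounds and keypad presses through server events, refreshes replicated door and keypad states at startup, and passes GameMode door save data to the client.
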(event Custom|Server_InteractRemote
  (params (RemoteRef :type BP%20Master%20Remote%20Object%20Reference))
  ;[1 1 1] Interact from Remote actor (Server)
  (Utilities|MyHasAuthority
    (:Server
      (Default|OnServeronInteract RemoteRef))))

(event Custom|Server_CallSetIsLockedDoor
  (params (DoorRef :type BP%20Master%20Door%20Object%20Reference) (IsLocked? :type Boolean))
  ;[1 1 1] Set door is locked (From interact | Server)
  (Default|OnServerSetIsLockedDoor DoorRef IsLocked? false))

(event Custom|Multi_PlaySoundAtLocation
  (params (Sound :type Sound%20Base%20Object%20Reference) (Location :type Vector))
  ;[1 1 1] Play sound at location (Server -> Multi)
  (Audio|PlaySoundatLocation Sound Location))

(event Custom|Server_DestroyActor
  (params (ActorRef :type Actor%20Object%20Reference))
  ;[1 1 1] Destroy an actor (Server)
  (Utilities|MyHasAuthority
    (:Server
      (Utilities|IsValid ActorRef
        (:Is%20Valid
          (Actor|DestroyActor ActorRef))))))

(event Custom|OnInteractPressed
  ;[1 1 1] On interact pressed
  (Traitement|Interact|OnInteract))

(event Custom|Client_RefreshDoorVariable
  (params (IsDoorLocked? :type Boolean) (Target :type BP%20Master%20Door%20Object%20Reference))
  ;[1 1 1] Refresh variable at startup otherwise they are not loaded correctly... (Be sure)
  (Variables|/Game/AntizeKitSystem/AntizeSystems/DoorSystem/Blueprints/Door/BP_MasterDoor.BP_MasterDoor_C|SetIsDoorLocked? Target IsDoorLocked?))

(event Custom|Server_CallOnButtonPressed
  (params (KeyPadRef :type BP%20Master%20Key%20Pad%20Object%20Reference) (Digit :type Integer))
  ;[1 1 1] Button Pressed (From W_KeyPad -> ButtonPressed | Server)
  (Utilities|MyHasAuthority
    (:Server
      (Default|OnServeronButtonPressed (Variables|/Game/AntizeKitSystem/AntizeSystems/DoorSystem/Blueprints/Door/BP_MasterKeyPad.BP_MasterKeyPad_C|GetW_KeyPadRef KeyPadRef) Digit))))

(event Custom|Server_RefreshAllDoorVariables
  ;[1 1 1] Constructeur
  (Spawn|RefreshAllDoorVariable false)
  (Utilities|FlowControl|Delay 0.1)
  (Spawn|RefreshAllDoorVariable true))

(event Custom|Client_OnSave
  (params (DoorSave :type Array%20of%20S%20Door%20Saved%20Structures))
  ;[1 1 1] On Save - Get ddoor in GameMode  (Server -> GameMode -> Client)
  (CallFunction|SaveDoorData DoorSave))

(event Custom|Server_CallOpenCloseAuto
  (params (DoorRef :type BP%20Master%20Door%20Object%20Reference) (RemoteOpenAngle :type Float%20%28single-precision%29) (IsOpenned? :type Boolean))
  ;[1 1 1] OpenClose door (From auto mode | Server)
  (Utilities|MyHasAuthority
    (:Server
      (Utilities|IsValid DoorRef
        (:Is%20Valid
          (Default|OnServerOpenCloseAuto DoorRef RemoteOpenAngle IsOpenned?))))))

(event Custom|Server_PlaySoundAtLocation
  (params (Sound :type Sound%20Base%20Object%20Reference) (Location :type Vector))
  ;[1 1 1] Play sound at location (Server -> Multi)
  (Utilities|MyHasAuthority
    (:Server
      (CallFunction|MultiPlaySoundatLocation Sound Location))))

(event Custom|Server_OnSave
  ;[1 1 1] On Save - Get ddoor in GameMode  (Server -> GameMode -> Client)
  (Utilities|MyHasAuthority
    (:Server
      (bind _doorsaved (Class|BPDoorInterface|MSGGetDoorSaved(Message) (Game|GetGameMode)))
      (CallFunction|ClientonSave _doorsaved))
    (:Remote
      (Development|PrintString "Warning : \"DoorComponent -> Server_OnSave\" is executed on client !" true true "(R=1.000000,G=0.500000,B=0.000000,A=1.000000)" 15.0))))

(event Custom|Server_CallOpenClose
  (params (Target :type BP%20Master%20Door%20Object%20Reference) (RemoteOpenAngle :type Float%20%28single-precision%29))
  ;[1 1 1] OpenClose door (From interact | Server)
  (Utilities|MyHasAuthority
    (:Server
      (Default|OnServerOpenClose Target (Components|GetOwner) RemoteOpenAngle))))

(event Custom|Client_RefreshKeypadVariables
  (params (IsError? :type Boolean) (Target :type BP%20Master%20Key%20Pad%20Object%20Reference))
  ;[1 1 1] Refresh variable at startup otherwise they are not loaded correctly... (Be sure)
  (Variables|/Game/AntizeKitSystem/AntizeSystems/DoorSystem/Blueprints/Door/BP_MasterKeyPad.BP_MasterKeyPad_C|SetIsError? Target IsError?))

(event EventBeginPlay
  (bind _returnvalue (Components|GetOwner))
  ;[1 1 1] Constructeur
  (Utilities|IsValid _returnvalue :!label _label
    (:Is%20Valid
      (bind _aspawn (Utilities|Casting|CastToPawn _returnvalue))
      (if (Pawn|IsLocallyControlled _aspawn)
        (Utilities|Time|SetTimerbyFunctionName 0 "PlayerSight" 0.1 true)
        (Utilities|FlowControl|Delay 0.1)
        (CallFunction|ServerRefreshAllDoorVariables)))
    (:Is%20Not%20Valid
      (Utilities|FlowControl|Delay 0.1)
      (goto _label))))

(fn HaveItem
  (params (Item :type Data%20Table%20Row%20Handle%20Structure%20%28by%20ref%29))
  (bind _returnvalue (Components|GetOwner))
  (Utilities|IsValid _returnvalue
    (:Is%20Valid
      (bind _inventoryref (Class|BPAntizeInventoryInterface|MSGGetInventory(Message) _returnvalue))
      (Utilities|IsValid _inventoryref
        (:Is%20Valid
          (return (.ItemFound? (Default|GetHaveItem _inventoryref Item))))
        (:Is%20Not%20Valid
          _)))
    (:Is%20Not%20Valid
      _))
  (return false))

(fn OnInteract
  (bind _returnvalue (Components|GetOwner))
  (bind _returnvalue_2 (Components|GetOwner))
  (bind _returnvalue_3 (Components|GetOwner))
  (Utilities|IsValid (Variables|Traitement|GetActorInSight)
    (:Is%20Valid
      ;[1 1 1] Interact with a door actor (Result)
      (bind _asbp_master_door (Utilities|Casting|CastToBP_MasterDoor (Variables|Traitement|GetActorInSight))
        (:then
          (bind _output_get (LocalVariables|SetLocal_DoorRef _asbp_master_door))
          (switch Utilities|FlowControl|Switch|SwitchonE_DoorState (Default|GetCanInteract _output_get self)
            (:NewEnumerator0
              ;[1 1 1] Door is open
              (bind _returnvalue_4 (Default|RefreshDoorAngle (LocalVariables|GetLocal_DoorRef)))
              (CallFunction|ServerCallOpenClose (LocalVariables|GetLocal_DoorRef) _returnvalue_4)
              (return))
            (:NewEnumerator4
              ;[1 1 1] Door is locked
              (Utilities|IsValid _returnvalue
                (:Is%20Valid
                  (bind _inventoryref (Class|BPAntizeInventoryInterface|MSGGetInventory(Message) _returnvalue))
                  (Default|ShowMessage _inventoryref true (select (or (Utilities|Enum|Equal(Enum) (Variables|/Game/AntizeKitSystem/AntizeSystems/DoorSystem/Blueprints/Door/BP_MasterDoor.BP_MasterDoor_C|GetSecutity (LocalVariables|GetLocal_DoorRef)) "NewEnumerator5") (Utilities|Enum|Equal(Enum) (Variables|/Game/AntizeKitSystem/AntizeSystems/DoorSystem/Blueprints/Door/BP_MasterDoor.BP_MasterDoor_C|GetSecutity (LocalVariables|GetLocal_DoorRef)) "NewEnumerator6")) "Locked from the other side." "This door is locked.")))
                (:Is%20Not%20Valid
                  _))
              (CallFunction|ServerPlaySoundatLocation "/Game/AntizeKitSystem/AntizeSystems/DoorSystem/Ressources/Audio/Cue_IsLocked.Cue_IsLocked" (Transformation|GetActorLocation (LocalVariables|GetLocal_DoorRef)))
              (return))
            (:NewEnumerator2
              ;[1 1 1] Unlock the door
              (CallFunction|ServerCallSetIsLockedDoor (LocalVariables|GetLocal_DoorRef) false)
              (Utilities|IsValid _returnvalue_2
                (:Is%20Valid
                  (bind _inventoryref_2 (Class|BPAntizeInventoryInterface|MSGGetInventory(Message) _returnvalue_2))
                  (Default|ShowMessage _inventoryref_2 true "This door is now unlocked.")
                  (return))
                (:Is%20Not%20Valid
                  (return))))
            (:NewEnumerator1
              ;[1 1 1] Lock the door
              (CallFunction|ServerCallSetIsLockedDoor (LocalVariables|GetLocal_DoorRef) true)
              (Utilities|IsValid _returnvalue_3
                (:Is%20Valid
                  (bind _inventoryref_3 (Class|BPAntizeInventoryInterface|MSGGetInventory(Message) _returnvalue_3))
                  (Default|ShowMessage _inventoryref_3 true "This door is now locked.")
                  (return))
                (:Is%20Not%20Valid
                  (return))))))
        (:CastFailed
          ;[1 1 1] Interact with a remote actor
          (bind _asbp_master_remote (Utilities|Casting|CastToBP_MasterRemote (Variables|Traitement|GetActorInSight))
            (:then
              (LocalVariables|SetLocal_RemoteInSight _asbp_master_remote)
              (Variables|/Game/AntizeKitSystem/AntizeSystems/DoorSystem/Blueprints/Door/BP_MasterRemote.BP_MasterRemote_C|SetDoorCompRef (LocalVariables|GetLocal_RemoteInSight) self)
              (CallFunction|ServerInteractRemote (LocalVariables|GetLocal_RemoteInSight))
              (return))
            (:CastFailed
              (return))))))
    (:Is%20Not%20Valid
      (return))))

(fn PlayerSight
  (bind _cameraref (Variables|Default|GetCameraRef))
  (bind _returnvalue (Transformation|GetWorldLocation _cameraref))
  ;[1 1 1] Check if an interactive actor is in the player's sight
  (Utilities|GetCamera
    (:Is%20Valid
      (bind (_outhit _returnvalue_2) (Collision|LineTraceByChannel _returnvalue (+ _returnvalue (* (Math|Vector|GetForwardVector _cameraref) 2e+02)) "TraceTypeQuery1" false 0 "None"))
      (if _returnvalue_2
        (Utilities|IsValid (.HitActor (Collision|BreakHitResult _outhit))
          (:Is%20Valid
            (LocalVariables|SetLocal_HitActor (.HitActor (Collision|BreakHitResult _outhit)))
            (LocalVariables|SetLocal_HitComp (.HitComponent (Collision|BreakHitResult _outhit)))
            (bind _asbp_master_door (Utilities|Casting|CastToBP_MasterDoor (LocalVariables|GetLocal_HitActor))
              (:then
                (if (!= _asbp_master_door (Variables|Traitement|GetActorInSight))
                  (Default|UpdateDoorInteraction _asbp_master_door "NewEnumerator0" (LocalVariables|GetLocal_HitComp))
                  (else
                    (return))))
              (:CastFailed
                (bind _asbp_master_remote (Utilities|Casting|CastToBP_MasterRemote (LocalVariables|GetLocal_HitActor))
                  (:then
                    (if (!= _asbp_master_remote (Variables|Traitement|GetActorInSight))
                      (Default|UpdateInteraction _asbp_master_remote "NewEnumerator0")
                      (else
                        (return))))
                  (:CastFailed
                    (OnTimer|ClearOldActor)
                    (return)))))
            (OnTimer|ClearOldActor)
            (Variables|Traitement|SetActorInSight (LocalVariables|GetLocal_HitActor))
            (return))
          (:Is%20Not%20Valid
            _)))
      (OnTimer|ClearOldActor)
      (return))))

(fn LeftButtonPressed
  (params (WidgetInteractionRef :type Widget%20Interaction%20Component%20Object%20Reference))
  ;[1 1 1] If a widget is hovered send the action and return if an action has been done.
  (Utilities|IsValid (Class|WidgetInteractionComponent|GetHoveredWidgetComponent WidgetInteractionRef)
    (:Is%20Valid
      (Class|WidgetInteractionComponent|PressPointerKey WidgetInteractionRef "LeftMouseButton")
      (if (>= (CallFunction|MyGetEngineVersion) 5)
        (bind _controllerref (Utilities|GetController)
          (:Is%20Valid
            (Input|SetInputModeGameOnly _controllerref))
          (:Is%20Not%20Valid
            _)))
      (return false))
    (:Is%20Not%20Valid
      (return true))))

(fn LeftButtonReleased
  (params (WidgetInteractionRef :type Widget%20Interaction%20Component%20Object%20Reference))
  ;[1 1 1] If a widget is hovered send the action and return if an action has been done.
  (Utilities|IsValid (Class|WidgetInteractionComponent|GetHoveredWidgetComponent WidgetInteractionRef)
    (:Is%20Valid
      (Class|WidgetInteractionComponent|ReleasePointerKey WidgetInteractionRef "LeftMouseButton")
      (return false))
    (:Is%20Not%20Valid
      (return true))))

(fn HoveredWidget
  (params (WidgetCompRef :type Widget%20Component%20Object%20Reference))
  ;[1 1 1] Hovered a widget from the character and set the component reference to the widget if valid.
  (Utilities|IsValid WidgetCompRef
    (:Is%20Valid
      (bind _asw_key_pad (Utilities|Casting|CastToW_KeyPad (UserInterface|GetUserWidgetObject WidgetCompRef))
        (:then
          (Default|SetDoorCompRef _asw_key_pad self))
        (:CastFailed
          _)))
    (:Is%20Not%20Valid
      _))
  (return))

(fn ClearOldActor
  (Utilities|IsValid (Variables|Traitement|GetActorInSight)
    (:Is%20Valid
      (bind _asbp_master_door (Utilities|Casting|CastToBP_MasterDoor (Variables|Traitement|GetActorInSight))
        (:then
          (Default|UpdateDoorInteraction _asbp_master_door "NewEnumerator1"))
        (:CastFailed
          (bind _asbp_master_remote (Utilities|Casting|CastToBP_MasterRemote (Variables|Traitement|GetActorInSight))
            (:then
              (Default|UpdateInteraction _asbp_master_remote "NewEnumerator1"))
            (:CastFailed
              (Variables|Traitement|SetActorInSight 0)
              (return)))))
      (Variables|Traitement|SetActorInSight 0)
      (return))
    (:Is%20Not%20Valid
      (return))))

(fn RefreshAllDoorVariable
  (params (OnServer? :type Boolean))
  ;[1 1 1] Refresh variables at startup otherwise they are not loaded correctly...
  (Utilities|MyHasAuthority
    (:Server
      (bind _outactors (Actor|GetAllActorsOfClass "/Game/AntizeKitSystem/AntizeSystems/DoorSystem/Blueprints/Door/BP_MasterKeyPad.BP_MasterKeyPad_C"))
      (for _array_element _outactors
        (Utilities|IsValid _array_element
          (:Is%20Valid
            (if (not OnServer?)
              (CallFunction|ClientRefreshKeypadVariables (Variables|/Game/AntizeKitSystem/AntizeSystems/DoorSystem/Blueprints/Door/BP_MasterKeyPad.BP_MasterKeyPad_C|GetIsError? _array_element) _array_element)))))
      (bind _outactors_2 (Actor|GetAllActorsOfClass "/Game/AntizeKitSystem/AntizeSystems/DoorSystem/Blueprints/Door/BP_MasterDoor.BP_MasterDoor_C"))
      (for _array_element_2 _outactors_2
        (Utilities|IsValid _array_element_2
          (:Is%20Valid
            (if OnServer?
              (Default|OnServerSetIsLockedDoor _array_element_2 (Variables|/Game/AntizeKitSystem/AntizeSystems/DoorSystem/Blueprints/Door/BP_MasterDoor.BP_MasterDoor_C|GetIsDoorLocked? _array_element_2) true)
              (else
                (CallFunction|ClientRefreshDoorVariable (Variables|/Game/AntizeKitSystem/AntizeSystems/DoorSystem/Blueprints/Door/BP_MasterDoor.BP_MasterDoor_C|GetIsDoorLocked? _array_element_2) _array_element_2))))))
      (return))))