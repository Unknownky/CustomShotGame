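; Function library for the multiplayer ping system, covering team membership, system pings and per-ping-type presentation data.
; JoinTeam prunes stale members, assigns a free slot that doubles as color ID, then clears pings and refreshes team icons through each pawn's BP_PingComponent.
; AddPingSystem sends system pings to one or all listed players under random IDs, and RemovePingSystem clears them.
; Select-based getters centralize scale, opacity, color, texture and sound.
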(fn GetColorbyID
  (params (ColorID :type Integer))
  (return (Utilities|Select :Index ColorID :Option%200 "(R=1.000000,G=0.250000,B=0.000000,A=1.000000)" :Option%201 "(R=0.000000,G=0.250000,B=1.000000,A=1.000000)" :Option%202 "(R=1.000000,G=0.000000,B=0.250000,A=1.000000)" :Option%203 "(R=0.250000,G=1.000000,B=0.000000,A=1.000000)" :Option%204 "(R=1.000000,G=0.132595,B=0.092793,A=1.000000)")))

(fn JoinTeam
  (params (PlayerRef :type Controller%20Object%20Reference) (OldTeamID :type Integer) (ToTeamID :type Integer) (AllTeam :type Array%20of%20S%20Team%20Structures))
  (LocalVariables|SetLocal_PlayerRef PlayerRef)
  (LocalVariables|SetLocal_OldTeamID OldTeamID)
  (LocalVariables|SetLocal_ToTeamID ToTeamID)
  (LocalVariables|SetLocal_AllTeam AllTeam)
  (bind (_success_ _pingcomprref) (AntizePing|Dev|GetPingCompRef (LocalVariables|GetLocal_PlayerRef)))
  (if _success_
    (bind _output_get (LocalVariables|SetLocal_PlayerPingCompRef _pingcomprref))
    ;[1 1 1] Don't continue if already in the Team
    (if (and (!= (.TeamID (Default|GetTeamID _output_get)) (LocalVariables|GetLocal_ToTeamID)) (!= (LocalVariables|GetLocal_OldTeamID) (LocalVariables|GetLocal_ToTeamID)))
      ;[1 1 1] Clean and get players in the old team
      (bind (_playerref _newallteam) (AntizePing|JoinTeam|CleanandGetPlayerinTeam (LocalVariables|GetLocal_AllTeam) (LocalVariables|GetLocal_PlayerRef) (LocalVariables|GetLocal_OldTeamID)))
      (LocalVariables|SetLocal_OldTeam _playerref)
      (LocalVariables|SetLocal_AllTeam _newallteam)
      ;[1 1 1] Remove all pings of the old team on the client
      (for _array_element (LocalVariables|GetLocal_OldTeam)
        (bind _playerid (Class|BPAntizeKitInterface|MSGAntizeGetPlayerID(Message) _array_element))
        (Default|ServerTryRemovePing (LocalVariables|GetLocal_PlayerPingCompRef) _playerid -1 false))
      ;[1 1 1] Remove all pings of the player on the client (Team keep ping)
      (Default|ServerTryRemovePing (LocalVariables|GetLocal_PlayerPingCompRef) (Default|GetPlayerID (LocalVariables|GetLocal_PlayerPingCompRef)) (.ColorID (Default|GetTeamID (LocalVariables|GetLocal_PlayerPingCompRef))) false)
      ;[1 1 1] Remove all team markers (Client and player team)
      (AntizePing|JoinTeam|RefreshTeamIcons (LocalVariables|GetLocal_OldTeam))
      (Default|ServerRefreshTeamIcons (LocalVariables|GetLocal_PlayerPingCompRef) false (Utilities|Array|MakeArray))
      (if (Utilities|Array|IsValidIndex (LocalVariables|GetLocal_AllTeam) (LocalVariables|GetLocal_ToTeamID))
        ;[1 1 1] Get player in the new team
        (bind _playerref_2 (AntizePing|JoinTeam|CleanandGetPlayerinTeam (LocalVariables|GetLocal_AllTeam) 0 (LocalVariables|GetLocal_ToTeamID)))
        (LocalVariables|SetLocal_NewTeam _playerref_2)
        ;[1 1 1] Search a free key in the team
        (bind _index (Utilities|FlowControl|ForLoopwithBreak 0 (LocalVariables|GetArrayTeamMaxSize) :!label _label)
          (:LoopBody
            (bind _output_get_2 (LocalVariables|SetLocal_KeyFound _index))
            (if (not (.ReturnValue (Utilities|Map|Find (Utilities|Struct|BreakS_Team (Utilities|Array|Get(acopy) (LocalVariables|GetLocal_AllTeam) (LocalVariables|GetLocal_ToTeamID))) _output_get_2)))
              (LocalVariables|SetLocal_KeyFound? true)
              (goto _label Break)))
          (:Completed
            ;[1 1 1] If free key is found add the player in the team
            (if (LocalVariables|GetLocal_KeyFound?)
              (Utilities|Map|Add (Utilities|Struct|BreakS_Team (Utilities|Array|Get(acopy) (LocalVariables|GetLocal_AllTeam) (LocalVariables|GetLocal_ToTeamID))) (LocalVariables|GetLocal_KeyFound) (LocalVariables|GetLocal_PlayerRef))
              (Default|ServerSetTeamID (LocalVariables|GetLocal_PlayerPingCompRef) (LocalVariables|GetLocal_ToTeamID) (LocalVariables|GetLocal_KeyFound))
              ;;[1 1 1] Refresh team marker (Client and player team)
              (Utilities|Array|AddUnique (LocalVariables|GetLocal_NewTeam) (LocalVariables|GetLocal_PlayerRef))
              (AntizePing|JoinTeam|RefreshTeamIcons (LocalVariables|GetLocal_NewTeam))
              (return (LocalVariables|GetLocal_AllTeam))
              (else
                (Default|ServerSetTeamID (LocalVariables|GetLocal_PlayerPingCompRef) -1)
                (Development|PrintString 0 "No empty slot found" true true "(R=1.000000,G=0.000000,B=0.000000,A=1.000000)" 1e+01)
                (return (LocalVariables|GetLocal_AllTeam))))))
        (else
          ;[1 1 1] Create a new row (If index is valid)
          (if (>= (LocalVariables|GetLocal_ToTeamID) 0)
            (Utilities|Array|SetArrayElem (LocalVariables|GetLocal_AllTeam) (LocalVariables|GetLocal_ToTeamID) (Utilities|Struct|MakeS_Team (Utilities|Map|MakeMap 0 (LocalVariables|GetLocal_PlayerRef))) true))
          (Default|ServerSetTeamID (LocalVariables|GetLocal_PlayerPingCompRef) (LocalVariables|GetLocal_ToTeamID))
          (return (LocalVariables|GetLocal_AllTeam))))
      (else
        (return (LocalVariables|GetLocal_AllTeam))))
    (else
      (return (LocalVariables|GetLocal_AllTeam)))))

(fn CleanandGetPlayerinTeam
  (params (AllTeam :type Array%20of%20S%20Team%20Structures) (PlayerToRemoveRef :type Controller%20Object%20Reference) (TeamID :type Integer))
  ;[1 1 1] Clean TeamID row
  (LocalVariables|SetLocal_AllTeam AllTeam)
  (LocalVariables|SetLocal_PlayerToRemoveRef PlayerToRemoveRef)
  (bind _output_get (LocalVariables|SetLocal_TeamID TeamID))
  (if (>= _output_get 0)
    (bind _keys (Utilities|Map|Keys (Utilities|Struct|BreakS_Team (Utilities|Array|Get(acopy) (LocalVariables|GetLocal_AllTeam) (LocalVariables|GetLocal_TeamID)))))
    (for _array_element _keys
      (bind _output_get_2 (LocalVariables|SetLocal_Key _array_element))
      (Utilities|IsValid (.Value (Utilities|Map|Find (Utilities|Struct|BreakS_Team (Utilities|Array|Get(acopy) (LocalVariables|GetLocal_AllTeam) (LocalVariables|GetLocal_TeamID))) _output_get_2))
        (:Is%20Valid
          (bind _teamid (Class|BPAntizeChatInterface|MSGGetTeamID(Message) (.Value (Utilities|Map|Find (Utilities|Struct|BreakS_Team (Utilities|Array|Get(acopy) (LocalVariables|GetLocal_AllTeam) (LocalVariables|GetLocal_TeamID))) _output_get_2))))
          (if (== _teamid (LocalVariables|GetLocal_TeamID))
            (Utilities|IsValid (LocalVariables|GetLocal_PlayerToRemoveRef)
              (:Is%20Valid
                (if (!= (LocalVariables|GetLocal_PlayerToRemoveRef) (.Value (Utilities|Map|Find (Utilities|Struct|BreakS_Team (Utilities|Array|Get(acopy) (LocalVariables|GetLocal_AllTeam) (LocalVariables|GetLocal_TeamID))) _output_get_2)))
                  (Utilities|Array|AddUnique (LocalVariables|GetLocal_PlayersRef) (.Value (Utilities|Map|Find (Utilities|Struct|BreakS_Team (Utilities|Array|Get(acopy) (LocalVariables|GetLocal_AllTeam) (LocalVariables|GetLocal_TeamID))) _output_get_2)) :!label _label)
                  (else
                    (Utilities|Map|Remove (Utilities|Struct|BreakS_Team (Utilities|Array|Get(acopy) (LocalVariables|GetLocal_AllTeam) (LocalVariables|GetLocal_TeamID))) (LocalVariables|GetLocal_Key) :!label _label_2))))
              (:Is%20Not%20Valid
                (goto _label)))
            (else
              (goto _label_2))))
        (:Is%20Not%20Valid
          (goto _label_2)))))
  (return (LocalVariables|GetLocal_PlayersRef) (LocalVariables|GetLocal_AllTeam)))

(fn RefreshTeamIcons
  (params (PlayersRef :type Array%20of%20Controller%20Object%20References))
  ;[1 1 1] Create the TeamMarker array to get the correct ID
  (for _array_element PlayersRef
    (bind _output_get (LocalVariables|SetLocal_PlayerRef _array_element))
    (Utilities|IsValid _output_get
      (:Is%20Valid
        (Utilities|IsValid (Pawn|GetControlledPawn (LocalVariables|GetLocal_PlayerRef))
          (:Is%20Valid
            (bind (_teamid _color_id) (Class|BPAntizeChatInterface|MSGGetTeamID(Message) (Pawn|GetControlledPawn (LocalVariables|GetLocal_PlayerRef))))
            (Utilities|Array|Add (LocalVariables|GetLocal_TeamIcons) (Utilities|Struct|MakeS_TeamIcons (Pawn|GetControlledPawn (LocalVariables|GetLocal_PlayerRef)) _teamid _color_id)))))))
  ;[1 1 1] Refresh team marker on client
  (for _array_element_2 PlayersRef
    (bind (_success_ _pingcomprref) (AntizePing|Dev|GetPingCompRef _array_element_2))
    (if _success_
      (Default|ServerRefreshTeamIcons _pingcomprref false (LocalVariables|GetLocal_TeamIcons))))
  (return))

(fn RemovePingSystem
  (params (PlayerRef :type Array%20of%20Controller%20Object%20References) (All? :type Boolean) (PingID :type Integer))
  ;[1 1 1] Remove all ping system
  (for _array_element PlayerRef
    (bind (_success_ _pingcomprref) (AntizePing|Dev|GetPingCompRef _array_element))
    (if _success_
      (Default|RemovePingSystem _pingcomprref PingID false All?)))
  (return))

(fn AddPingSystem
  (params (PlayerRef :type Array%20of%20Controller%20Object%20References) (ActualRandomPing :type Array%20of%20Integers) (ToPlayerID :type Integer) (Location :type Vector))
  (LocalVariables|SetLocal_Everyone? (< ToPlayerID 0))
  (bind _systemid (AntizePing|Dev|GetSystemID ActualRandomPing))
  (LocalVariables|SetLocal_SystemID _systemid)
  (bind _array_element (Utilities|Array|ForEachLoopwithBreak PlayerRef :!label _label)
    (:LoopBody
      (bind (_success_ _pingcomprref) (AntizePing|Dev|GetPingCompRef _array_element))
      (if _success_
        (if (or (LocalVariables|GetLocal_Everyone?) (== ToPlayerID (Default|GetPlayerID _pingcomprref)))
          (Default|ClientCallReceivePing _pingcomprref Location "NewEnumerator4" 0 (LocalVariables|GetLocal_SystemID) -1 4 true)
          (if (not (LocalVariables|GetLocal_Everyone?))
            (goto _label Break)))))
    (:Completed
      (return (LocalVariables|GetLocal_SystemID)))))

(fn GetSystemID
  (params (ActualRandomPing :type Array%20of%20Integers))
  (bind _returnvalue (Math|Random|RandomIntegerinRange 500 999999999))
  (LocalVariables|SetLocal_SystemID _returnvalue :!label _label)
  (if (Utilities|Array|ContainsItem ActualRandomPing _returnvalue)
    (bind _result (Math|Integer|IncrementInt (LocalVariables|GetLocal_Attempt))
      (:%20%20
        (if (< _result 500)
          (goto _label)
          (else
            (return (Math|Random|RandomIntegerinRange 500 999999999))))))
    (else
      (Utilities|Array|Add ActualRandomPing (LocalVariables|GetLocal_SystemID))
      (return (LocalVariables|GetLocal_SystemID)))))

(fn GetPingCompRef
  (params (ControllerRef :type Controller%20Object%20Reference))
  (bind _returnvalue (Pawn|GetControlledPawn ControllerRef))
  (bind _returnvalue_2 (Actor|GetComponentbyClass _returnvalue "/Game/AntizeKitSystem/AntizeSystems/SimplePingSystem/Blueprints/BP_PingComponent.BP_PingComponent_C"))
  (Utilities|IsValid ControllerRef
    (:Is%20Valid
      (Utilities|IsValid _returnvalue
        (:Is%20Valid
          (Utilities|IsValid _returnvalue_2
            (:Is%20Valid
              (return true _returnvalue_2))
            (:Is%20Not%20Valid
              _)))
        (:Is%20Not%20Valid
          _)))
    (:Is%20Not%20Valid
      _))
  (return false 0))

(fn DoRequestPlayerID
  (params (NewParam :type Integer%20%28by%20ref%29))
  (LocalVariables|SetLocal_PlayerID NewParam)
  (Math|Integer|IncrementInt NewParam
    (:%20%20
      (return (LocalVariables|GetLocal_PlayerID)))))

(fn GetScaleData
  (params (PingType :type E_PingType%20Enum :default "NewEnumerator1"))
  (return (Utilities|Select :Index PingType :NewEnumerator1 true :NewEnumerator0 true :NewEnumerator3 true :NewEnumerator5 true :NewEnumerator7 true :NewEnumerator4 true :NewEnumerator8 true) (Utilities|Select :Index PingType :NewEnumerator1 true :NewEnumerator0 true :NewEnumerator3 true :NewEnumerator5 true :NewEnumerator7 true :NewEnumerator4 true :NewEnumerator8 true) (Utilities|Select :Index PingType :NewEnumerator1 0.65 :NewEnumerator0 0.65 :NewEnumerator3 0.65 :NewEnumerator5 0.65 :NewEnumerator7 0.5 :NewEnumerator4 0.5 :NewEnumerator8 0.5) (Utilities|Select :Index PingType :NewEnumerator1 0.75 :NewEnumerator0 0.75 :NewEnumerator3 0.75 :NewEnumerator5 0.75 :NewEnumerator7 0.75 :NewEnumerator4 0.75 :NewEnumerator8 0.75) (Utilities|Select :Index PingType :NewEnumerator1 2.25e+03 :NewEnumerator0 2.25e+03 :NewEnumerator3 2.25e+03 :NewEnumerator5 2.25e+03 :NewEnumerator7 2.25e+03 :NewEnumerator4 2.25e+03 :NewEnumerator8 2.25e+03) (Utilities|Select :Index PingType :NewEnumerator1 5e+03 :NewEnumerator0 5e+03 :NewEnumerator3 5e+03 :NewEnumerator5 5e+03 :NewEnumerator7 5e+03 :NewEnumerator4 5e+03 :NewEnumerator8 5e+03)))

(fn GetOpacityData
  (params (PingType :type E_PingType%20Enum :default "NewEnumerator1"))
  (return (Utilities|Select :Index PingType :NewEnumerator1 true :NewEnumerator0 true :NewEnumerator3 true :NewEnumerator5 true :NewEnumerator7 true :NewEnumerator4 true :NewEnumerator8 true) (Utilities|Select :Index PingType :NewEnumerator1 true :NewEnumerator0 true :NewEnumerator3 true :NewEnumerator5 true :NewEnumerator7 true :NewEnumerator4 true :NewEnumerator8 true) (Utilities|Select :Index PingType :NewEnumerator1 0.75 :NewEnumerator0 0.75 :NewEnumerator3 0.75 :NewEnumerator5 0.75 :NewEnumerator7 0.75 :NewEnumerator4 0.75 :NewEnumerator8 0.75) (Utilities|Select :Index PingType :NewEnumerator1 0.9 :NewEnumerator0 0.9 :NewEnumerator3 0.9 :NewEnumerator5 0.9 :NewEnumerator7 0.9 :NewEnumerator4 0.9 :NewEnumerator8 0.9) (Utilities|Select :Index PingType :NewEnumerator1 2.5e+03 :NewEnumerator0 2.5e+03 :NewEnumerator3 2.5e+03 :NewEnumerator5 2.5e+03 :NewEnumerator7 2.5e+03 :NewEnumerator4 2.5e+03 :NewEnumerator8 2.5e+03) (Utilities|Select :Index PingType :NewEnumerator1 8.5e+03 :NewEnumerator0 8.5e+03 :NewEnumerator3 8.5e+03 :NewEnumerator5 8.5e+03 :NewEnumerator7 8.5e+03 :NewEnumerator4 8.5e+03 :NewEnumerator8 8.5e+03)))

(fn GetColorData
  (params (PingType :type E_PingType%20Enum :default "NewEnumerator1") (ColorID :type Integer))
  (bind _color (AntizePing|Dev|GetColorbyID ColorID))
  (bind _returnvalue (Utilities|Select :Index PingType :NewEnumerator1 _color :NewEnumerator0 "(R=1.000000,G=0.007843,B=0.000000,A=1.000000)" :NewEnumerator3 "(R=1.000000,G=0.007843,B=0.000000,A=1.000000)" :NewEnumerator5 _color :NewEnumerator7 "(R=1.000000,G=1.000000,B=1.000000,A=1.000000)" :NewEnumerator4 "(R=0.380392,G=1.000000,B=0.831373,A=1.000000)" :NewEnumerator8 "(R=1.000000,G=0.317647,B=0.000000,A=1.000000)"))
  (bind (_r _g _b) (Utilities|Struct|BreakLinearColor _returnvalue))
  (return (Utilities|Struct|MakeLinearColor _r _g _b 0.55)))

(fn GetTextureData
  (params (PingType :type E_PingType%20Enum :default "NewEnumerator1"))
  (return (Utilities|Select :Index PingType :NewEnumerator1 "/Game/AntizeKitSystem/AntizeSystems/SimplePingSystem/Textures/T_PingInfo.T_PingInfo" :NewEnumerator0 "/Game/AntizeKitSystem/AntizeSystems/SimplePingSystem/Textures/T_PingEnemy.T_PingEnemy" :NewEnumerator3 "/Game/AntizeKitSystem/AntizeSystems/SimplePingSystem/Textures/T_PingEnemyFollow.T_PingEnemyFollow" :NewEnumerator5 "/Game/AntizeKitSystem/AntizeSystems/SimplePingSystem/Textures/T_PingOverEmpty.T_PingOverEmpty" :NewEnumerator7 "/Game/AntizeKitSystem/AntizeSystems/SimplePingSystem/Textures/T_Base.T_Base" :NewEnumerator4 "/Game/AntizeKitSystem/AntizeSystems/SimplePingSystem/Textures/T_PingOver.T_PingOver" :NewEnumerator8 "/Game/AntizeKitSystem/AntizeSystems/SimplePingSystem/Textures/T_Marker.T_Marker")))

(fn GetSoundData
  (params (PingType :type E_PingType%20Enum :default "NewEnumerator1"))
  (return (Utilities|Select :Index PingType :NewEnumerator1 "/Game/AntizeKitSystem/AntizeSystems/SimplePingSystem/Audio/Cue_OnPing.Cue_OnPing" :NewEnumerator0 "/Game/AntizeKitSystem/AntizeSystems/SimplePingSystem/Audio/Cue_PingEnemySpotted.Cue_PingEnemySpotted" :NewEnumerator3 "/Game/AntizeKitSystem/AntizeSystems/SimplePingSystem/Audio/Cue_PingEnemyFollow.Cue_PingEnemyFollow" :NewEnumerator5 0 :NewEnumerator7 0 :NewEnumerator4 "/Game/AntizeKitSystem/AntizeSystems/SimplePingSystem/Audio/Cue_OnPing.Cue_OnPing" :NewEnumerator8 0)))

(fn GetCharRef
  (params (ControllerRef :type Controller%20Object%20Reference))
  (bind _returnvalue (Pawn|GetControlledPawn ControllerRef))
  (Utilities|IsValid ControllerRef
    (:Is%20Valid
      (Utilities|IsValid _returnvalue
        (:Is%20Valid
          (return true _returnvalue))
        (:Is%20Not%20Valid
          _)))
    (:Is%20Not%20Valid
      _))
  (return false 0))