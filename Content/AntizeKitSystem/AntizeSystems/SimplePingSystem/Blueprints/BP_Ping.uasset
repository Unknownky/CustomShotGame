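; World ping marker actor for the ping system, showing a typed, coloured W_Ping widget with distance to its owner.
; BeginPlay notifies the hit actor through interface messages, may take its texture, and times removal by type; Enemy Follow later becomes a free ping, detaches and traces to the floor.
; CalculeDistance refreshes meter, scale and opacity only on movement unless forced, closing orphaned pings.
; DoPingOnPing tracks other players' responses by colour ID.
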(event Custom|RefreshTexture
  (params (Texture :type Texture%202D%20Object%20Reference))
  ;[1 1 1] Refresh the texture (Only if texture valid)
  (Utilities|IsValid Texture
    (:Is%20Valid
      (Utilities|FlowControl|Delay 0.02)
      (Appearance|SetBrushfromTexture (Variables|/Game/AntizeKitSystem/AntizeSystems/SimplePingSystem/Widgets/W_Ping.W_Ping_C|GetImage_PingMarker (Variables|Spawn|GetW_PingRef)) Texture false))))

(event Custom|OnFade
  (params (DoFade? :type Boolean))
  ;[1 1 1] Fade animation
  (if (Math|Boolean|NotEqual(Boolean) DoFade? (Variables|Traitement|GetActualFade))
    (Variables|Traitement|SetActualFade DoFade?)
    (Utilities|IsValid (Variables|Spawn|GetW_PingRef)
      (:Is%20Valid
        (if (Variables|Traitement|GetActualFade)
          (bind _alpha (Timeline|Timeline_Fade Play)
            (:Update
              (Widget|SetRenderOpacity (Variables|/Game/AntizeKitSystem/AntizeSystems/SimplePingSystem/Widgets/W_Ping.W_Ping_C|GetMyOverlayFade (Variables|Spawn|GetW_PingRef)) (Math|Float|Lerp 1.0 0.2 _alpha))))
          (else
            (Timeline|Timeline_Fade Reverse)))))))

(event Custom|RemoveActorAfterTime
  (bind _pingtype (Variables|Spawn|GetPingType))
  ;[1 1 1] Remove actor after delay
  (if (and (Utilities|Enum|NotEqual(Enum) _pingtype "NewEnumerator7") (Utilities|Enum|NotEqual(Enum) _pingtype "NewEnumerator8"))
    (Utilities|FlowControl|Delay 2e+01)
    (Utilities|IsValid self
      (:Is%20Valid
        (CallFunction|DoOnceDestroyActor)))))

(event Custom|DoOnceDestroyActor
  (bind _w_pingref (Variables|Spawn|GetW_PingRef))
  ;[1 1 1] DestroyActor only called once
  (Utilities|FlowControl|DoOnce false
    (:Completed
      (Utilities|IsValid self
        (:Is%20Valid
          (Utilities|IsValid _w_pingref
            (:Is%20Valid
              (Default|ClosePing _w_pingref))
            (:Is%20Not%20Valid
              (Actor|DestroyActor))))))))

(event EventBeginPlay
  (bind _returnvalue (Transformation|GetActorLocation))
  ;[1 1 1] Constructeur
  (bind _asw_ping (Utilities|Casting|CastToW_Ping (UserInterface|GetUserWidgetObject (Variables|Default|GetWidget))))
  (Variables|Spawn|SetW_PingRef _asw_ping)
  (Default|RefreshPing (Variables|Spawn|GetW_PingRef) (Variables|Spawn|GetPingType) (Variables|Spawn|GetColorID))
  (Variables|/Game/AntizeKitSystem/AntizeSystems/SimplePingSystem/Widgets/W_Ping.W_Ping_C|SetPingRef (Variables|Spawn|GetW_PingRef) self)
  (Spawn|DisableCollision)
  (Utilities|IsValid (Variables|Spawn|GetActorHit)
    (:Is%20Valid
      (Class|BPAntizePingInterface|MSGPingAttachPingActor(Message) (Variables|Spawn|GetActorHit) (Variables|Spawn|GetPingType) self)
      (Update|CalculeDistance true)
      (switch Utilities|FlowControl|Switch|SwitchonE_PingType (Variables|Spawn|GetPingType)
        (:NewEnumerator1
          (bind _actortype (Class|BPAntizePingInterface|MSGPingGetActorType(Message) (Variables|Spawn|GetActorHit) :!label _label))
          (if (Utilities|Enum|Equal(Enum) _actortype "NewEnumerator2")
            ;[1 1 1] Set the ping on item location and get item texture
            (Variables|Spawn|SetKeepOnActorDestroy? false :!label _label_2)
            (bind _texture (Class|BPAntizePingInterface|MSGPingGetPingTexture(Message) (Variables|Spawn|GetActorHit)))
            (Default|RefreshPing (Variables|Spawn|GetW_PingRef) (Variables|Spawn|GetPingType) (Variables|Spawn|GetColorID) _texture)
            (CallFunction|RemoveActorAfterTime)
            (else
              (CallFunction|RemoveActorAfterTime))))
        (:NewEnumerator0
          (goto _label))
        (:NewEnumerator3
          ;[1 1 1] Attach the ping to an actor and detach after the delay (Only if not SystemAlly)
          (Utilities|FlowControl|Delay 4.0)
          (bind _output_get (Variables|Spawn|SetPingType "NewEnumerator1"))
          (Default|RefreshPing (Variables|Spawn|GetW_PingRef) _output_get (Variables|Spawn|GetColorID))
          (Update|CalculeDistance true)
          (Utilities|IsValid self
            (:Is%20Valid
              (Transformation|DetachFromActor "KeepWorld" "KeepWorld" "KeepWorld")
              (CallFunction|RemoveActorAfterTime)
              ;;[1 1 1] Try to set ping on floor
              (bind _outhit (Collision|LineTraceByChannel _returnvalue (- _returnvalue "0, 0,250.000000") "TraceTypeQuery1" false (Utilities|Array|MakeArray (Variables|Spawn|GetActorHit)) "None"))
              (if (.bBlockingHit (Collision|BreakHitResult _outhit))
                (if (Math|Vector|NotEqual(Vector) (.ImpactPoint (Collision|BreakHitResult _outhit)) "0, 0, 0" 0.0001)
                  (Transformation|SetActorLocation (.ImpactPoint (Collision|BreakHitResult _outhit)) false false))))))
        (:NewEnumerator5)
        (:NewEnumerator7
          (goto _label_2))
        (:NewEnumerator4
          (goto _label))
        (:NewEnumerator8)))
    (:Is%20Not%20Valid
      (CallFunction|RemoveActorAfterTime)
      (Update|CalculeDistance true))))

(fn ConstructionScript)

(fn CalculeDistance
  (params (Force? :type Boolean))
  (bind _lastselflocation (Variables|Traitement|GetLastSelfLocation))
  (bind _lastownerlocation (Variables|Traitement|GetLastOwnerLocation))
  (bind (_x _y) (Math|Vector|BreakVector _lastselflocation))
  (bind (_x_2 _y_2) (Math|Vector|BreakVector _lastownerlocation))
  ;[1 1 1] Check if actors are still valid
  (Utilities|IsValid self
    (:Is%20Valid
      (Utilities|IsValid (Variables|Spawn|GetOwnerRef)
        (:Is%20Valid
          (Utilities|IsValid (Variables|Spawn|GetActorHit)
            (:Is%20Valid
              (if (!= (Variables|Spawn|GetActorHit) (Variables|Spawn|GetOwnerRef))
                (Utilities|IsValid (Variables|Spawn|GetW_PingRef) :!label _label
                  (:Is%20Valid
                    (if Force?
                      ;[1 1 1] Force update location and metter
                      (Update|CheckSelfLocation)
                      (Update|CheckOwnerLocation)
                      (else
                        (switch Utilities|FlowControl|Switch|SwitchonE_PingType (Variables|Spawn|GetPingType)
                          (:NewEnumerator1
                            ;[1 1 1] Check if the owner location is not the same as the last refresh
                            (bind _different_ (Update|CheckOwnerLocation :!label _label_2))
                            (if _different_
                              _
                              (else
                                (return))))
                          (:NewEnumerator0
                            (goto _label_2))
                          (:NewEnumerator3
                            ;[1 1 1] If it's following an actor, check locations of player and ping
                            (bind _different__2 (Update|CheckSelfLocation :!label _label_3))
                            (bind _different__3 (Update|CheckOwnerLocation))
                            (if (or _different__3 _different__2)
                              _
                              (else
                                (return))))
                          (:NewEnumerator5
                            (goto _label_3))
                          (:NewEnumerator7
                            (goto _label_2))
                          (:NewEnumerator4
                            (goto _label_2))
                          (:NewEnumerator8
                            (goto _label_3)))))
                    (LocalVariables|SetLocal_Metter (Math|Vector|VectorLength (- (Math|Vector|MakeVector _x_2 _y_2 0.0) (Math|Vector|MakeVector _x _y 0.0))))
                    (Default|UpdateMeter (Variables|Spawn|GetW_PingRef) (LocalVariables|GetLocal_Metter))
                    (Default|ScaleonRange (Variables|Spawn|GetW_PingRef) (LocalVariables|GetLocal_Metter))
                    (Default|OpacityonRange (Variables|Spawn|GetW_PingRef) (LocalVariables|GetLocal_Metter))
                    (return))
                  (:Is%20Not%20Valid
                    _))))
            (:Is%20Not%20Valid
              (if (Variables|Spawn|GetKeepOnActorDestroy?)
                (goto _label)
                (else
                  (CallFunction|DoOnceDestroyActor :!label _label_4))))))
        (:Is%20Not%20Valid
          (goto _label_4))))
    (:Is%20Not%20Valid
      (goto _label_4)))
  (return))

(fn CheckSelfLocation
  (if (Math|Vector|NotEqual(Vector) (Variables|Traitement|GetLastSelfLocation) (Transformation|GetActorLocation self) 0.1)
    (Variables|Traitement|SetLastSelfLocation (Transformation|GetActorLocation self))
    (return true)
    (else
      (return false))))

(fn CheckOwnerLocation
  (if (Math|Vector|NotEqual(Vector) (Variables|Traitement|GetLastOwnerLocation) (Transformation|GetActorLocation (Variables|Spawn|GetOwnerRef)) 0.1)
    (Variables|Traitement|SetLastOwnerLocation (Transformation|GetActorLocation (Variables|Spawn|GetOwnerRef)))
    (return true)
    (else
      (return false))))

(fn DoPingonPing
  (params (Add? :type Boolean) (ColorID :type Integer) (PlaySound? :type Boolean))
  (LocalVariables|SetLocal_Add? Add?)
  (LocalVariables|SetLocal_ColorID ColorID)
  (if (and (!= (Variables|Spawn|GetColorID) (LocalVariables|GetLocal_ColorID)) (Utilities|Array|IsValidIndex (Variables|Traitement|GetActualPingOnPing) (LocalVariables|GetLocal_ColorID)))
    (if (Math|Boolean|NotEqual(Boolean) (Utilities|Array|Get(acopy) (Variables|Traitement|GetActualPingOnPing) (LocalVariables|GetLocal_ColorID)) (LocalVariables|GetLocal_Add?))
      (Utilities|IsValid (Variables|Spawn|GetW_PingRef)
        (:Is%20Valid
          (Default|SetPingonPingWidget (Variables|Spawn|GetW_PingRef) (LocalVariables|GetLocal_Add?) (LocalVariables|GetLocal_ColorID) PlaySound?)
          (Utilities|Array|SetArrayElem (Variables|Traitement|GetActualPingOnPing) (LocalVariables|GetLocal_ColorID) (LocalVariables|GetLocal_Add?) true)
          (return true))
        (:Is%20Not%20Valid
          _))))
  (return false))

(fn DisableCollision
  (bind _pingtype (Variables|Spawn|GetPingType))
  ;[1 1 1] Disable collision for these ping types
  (if (Math|Boolean|ORBoolean (Utilities|Enum|Equal(Enum) _pingtype "NewEnumerator5") (Utilities|Enum|Equal(Enum) _pingtype "NewEnumerator7") (Utilities|Enum|Equal(Enum) _pingtype "NewEnumerator4") (Utilities|Enum|Equal(Enum) _pingtype "NewEnumerator8"))
    (Collision|SetCollisionEnabled (Variables|Default|GetSphere) "NoCollision")))