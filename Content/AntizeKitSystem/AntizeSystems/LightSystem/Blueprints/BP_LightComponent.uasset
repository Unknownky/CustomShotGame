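; Player pawn component that lets a character interact with lights and light switches in the Antize light system.
; On the locally controlled pawn, a looping timer line-traces from the camera, toggling key prompts on interface actors and adding a center-screen widget.
; Overlapped light actors are tracked and sent opacity updates on movement input, throttled by a gate.
; Interactions route through the server to lights or switches, and sounds are relayed via server to multicast.
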(event Custom|EndOverlap
  (params (OtherActor :type Actor%20Object%20Reference))
  ;[1 1 1] (Client) Actor Begin/End overlap
  (bind _returnvalue (Utilities|Array|RemoveItem (Variables|Traitement|GetActorInRange) OtherActor))
  (if _returnvalue
    (Class|BPAntizeLightInterfaces|MSGLightSetOpacity(Message) OtherActor false 0 0.0)))

(event Custom|OnOverlap
  (params (OtherActor :type Actor%20Object%20Reference))
  ;[1 1 1] (Client) Actor Begin/End overlap
  (if (Utilities|DoesObjectImplementInterface OtherActor "/Game/AntizeKitSystem/AntizeSystems/LightSystem/Blueprints/Others/BP_AntizeLightInterfaces.BP_AntizeLightInterfaces_C")
    (Utilities|Array|AddUnique (Variables|Traitement|GetActorInRange) OtherActor)))

(event Custom|Server_PlaySound
  (params (Sound :type Sound%20Base%20Object%20Reference) (Location :type Vector))
  ;[1 1 1] Replicated -> Play sound at location
  (Utilities|MyHasAuthority
    (:Server
      (CallFunction|MultiPlaySound Sound Location))))

(event Custom|Server_Interact
  (params (ActorRef :type Actor%20Object%20Reference))
  ;[1 1 1] (Server) Interact with actor
  (Utilities|GetOwner
    (:Is%20Valid
      (Interact|OnServerInteract ActorRef))))

(event Custom|Multi_PlaySound
  (params (Sound :type Sound%20Base%20Object%20Reference) (Location :type Vector))
  ;[1 1 1] Replicated -> Play sound at location
  (Audio|SpawnSoundatLocation Sound Location))

(event Custom|CallPlaySound
  (params (Sound :type Sound%20Cue%20Object%20Reference) (Location :type Vector))
  ;[1 1 1] Replicated -> Play sound at location
  (CallFunction|ServerPlaySound Sound Location))

(event Custom|OnMoveY
  (params (AxisValue :type Float%20%28single-precision%29))
  ;[1 1 1] (Client - Optimized) Movement input
  (if (!= AxisValue 0.0)
    (Utilities|FlowControl|Sequence
      (:then_0
        (Utilities|FlowControl|Gate false :!label _label
          (:Exit
            (bind _aspawn (Utilities|GetOwner)
              (:Is%20Valid
                (for _array_element (Variables|Traitement|GetActorInRange)
                  (Class|BPAntizeLightInterfaces|MSGLightSetOpacity(Message) _array_element true _aspawn 0.0))
                (Utilities|FlowControl|Delay 0.05)
                (goto _label Open))))))
      (:then_1
        (goto _label Close)))))

(event Custom|OnMoveX
  (params (AxisValue :type Float%20%28single-precision%29))
  ;[1 1 1] (Client - Optimized) Movement input
  (if (and (== (stale Custom|OnMoveY AxisValue) 0.0) (!= AxisValue 0.0))
    (Utilities|FlowControl|Sequence
      (:then_0
        (Utilities|FlowControl|Gate false :!label _label
          (:Exit
            (bind _aspawn (Utilities|GetOwner)
              (:Is%20Valid
                (for _array_element (Variables|Traitement|GetActorInRange)
                  (Class|BPAntizeLightInterfaces|MSGLightSetOpacity(Message) _array_element true _aspawn 0.0))
                (Utilities|FlowControl|Delay 0.05)
                (goto _label Open))))))
      (:then_1
        (goto _label Close)))))

(event EventBeginPlay
  ;[1 1 1] Constructeur
  (bind _aspawn (Utilities|GetOwner)
    (:Is%20Valid
      (if (Pawn|IsLocallyControlled _aspawn)
        (Utilities|Time|SetTimerbyFunctionName 0 "OnLineTrace" 0.2 true)
        (bind _returnvalue (UserInterface|CreateWidget "/Game/AntizeKitSystem/AntizeSystems/LightSystem/Widgets/W_CenterScreen.W_CenterScreen_C"))
        (UserInterface|Viewport|AddtoViewport _returnvalue 0)))))

(fn OnLineTrace
  (bind _cameraref (Variables|Default|GetCameraRef))
  (bind _returnvalue (Transformation|GetWorldLocation _cameraref))
  ;[1 1 1] Check if actor on player sight
  (Utilities|GetCamera
    (:Is%20Valid
      (bind (_outhit _returnvalue_2) (Collision|LineTraceByChannel _returnvalue (+ _returnvalue (* (Math|Vector|GetForwardVector _cameraref) 2e+02)) "TraceTypeQuery1" false 0 "None" true "(R=1.000000,G=0.000000,B=0.000000,A=1.000000)" "(R=0.000000,G=1.000000,B=0.000000,A=1.000000)" 1.0))
      (if _returnvalue_2
        (Utilities|IsValid (.HitActor (Collision|BreakHitResult _outhit))
          (:Is%20Valid
            (if (Utilities|DoesObjectImplementInterface (.HitActor (Collision|BreakHitResult _outhit)) "/Game/AntizeKitSystem/AntizeSystems/LightSystem/Blueprints/Others/BP_AntizeLightInterfaces.BP_AntizeLightInterfaces_C")
              (Utilities|IsValid (Variables|Traitement|GetActorInLineTrace)
                (:Is%20Valid
                  (if (== (Variables|Traitement|GetActorInLineTrace) (.HitActor (Collision|BreakHitResult _outhit)))
                    (return)
                    (else
                      (Class|BPAntizeLightInterfaces|MSGLightonLinetraceChanged(Message) (Variables|Traitement|GetActorInLineTrace) false))))
                (:Is%20Not%20Valid
                  _))
              (bind _output_get (Variables|Traitement|SetActorInLineTrace (.HitActor (Collision|BreakHitResult _outhit))))
              (Class|BPAntizeLightInterfaces|MSGLightonLinetraceChanged(Message) _output_get true (Class|KismetInputLibrary|KeyGetDisplayName (Utilities|Struct|BreakInputActionKeyMapping (Variables|Settings|GetInteractKey))))
              (return)
              (else
                _)))
          (:Is%20Not%20Valid
            _)))
      ;;[1 1 1] HideText and delete ActorInLineTraceRef
      (Utilities|IsValid (Variables|Traitement|GetActorInLineTrace)
        (:Is%20Valid
          (Class|BPAntizeLightInterfaces|MSGLightonLinetraceChanged(Message) (Variables|Traitement|GetActorInLineTrace) false)
          (Variables|Traitement|SetActorInLineTrace 0)
          (return))))
    (:Is%20Not%20Valid
      (return))))

(fn OnInteract
  (bind _actorinlinetrace (Variables|Traitement|GetActorInLineTrace))
  (Utilities|IsValid _actorinlinetrace
    (:Is%20Valid
      (CallFunction|ServerInteract _actorinlinetrace)
      (return true))
    (:Is%20Not%20Valid
      (return false))))

(fn OnServerInteract
  (params (ActorRef :type Actor%20Object%20Reference))
  (LocalVariables|SetLocal_ActorRef ActorRef)
  (Utilities|MyHasAuthority
    (:Server
      (bind _asbp_master_light (Utilities|Casting|CastToBP_Master_Light (LocalVariables|GetLocal_ActorRef))
        (:then
          (Default|LightInteract _asbp_master_light false)
          (return))
        (:CastFailed
          (bind _asmaster_light_switch (Utilities|Casting|CastToMaster_LightSwitch (LocalVariables|GetLocal_ActorRef))
            (:then
              (bind _ascharacter (Utilities|Casting|CastToCharacter (Variables|Traitement|GetOwnerRef)))
              (Default|LightSwitchInteract _asmaster_light_switch _ascharacter)
              (return))
            (:CastFailed
              (return))))))
    (:Remote
      (return))))