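; Master light switch actor, configured as either an interactable Switcher or a Pawn-triggered CollisionBox, that controls linked lights.
; The server applies the Enabled state to linked and optional inverse lights and syncs linked switches; multicasts update the indicator color and prompt widget.
; Collision modes include normal, timed and on-only or off-only.
; The construction script configures components per type and cleans link arrays; prompts fade with distance and line-of-sight.
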(event OnComponentEndOverlap(CollisionBox)
  (params (OverlappedComponent :type Primitive%20Component%20Object%20Reference) (OtherActor :type Actor%20Object%20Reference) (OtherComp :type Primitive%20Component%20Object%20Reference) (OtherBodyIndex :type Integer))
  ;[1 1 1] (OnServer) Bengin/End overlap (Called by player collision)
  (Networking|SwitchHasAuthority
    (:Authority
      (if (Utilities|Enum|Equal(Enum) (Variables|Setting|GetLightSwitchType) "NewEnumerator1")
        (Utilities|IsValid OtherActor
          (:Is%20Valid
            (Utilities|Casting|CastToPawn OtherActor)
            (switch Utilities|FlowControl|Switch|SwitchonE_SwticherCollisionType (Variables|Setting|ColliionBox|GetCollisionBoxType)
              (:NewEnumerator5
                (if (Variables|Setting|GetEnabled?)
                  (Variables|Setting|SetEnabled? false)
                  (Traitement|OnServerEnableDisableLinkedLight true false))))))))))

(event OnComponentBeginOverlap(CollisionBox)
  (params (OverlappedComponent :type Primitive%20Component%20Object%20Reference) (OtherActor :type Actor%20Object%20Reference) (OtherComp :type Primitive%20Component%20Object%20Reference) (OtherBodyIndex :type Integer) (bFromSweep :type Boolean) (SweepResult :type Hit%20Result%20Structure%20%28by%20ref%29))
  ;[1 1 1] (OnServer) Bengin/End overlap (Called by player collision)
  (Networking|SwitchHasAuthority
    (:Authority
      (if (Utilities|Enum|Equal(Enum) (Variables|Setting|GetLightSwitchType) "NewEnumerator1")
        (Utilities|IsValid OtherActor
          (:Is%20Valid
            (Utilities|Casting|CastToPawn OtherActor)
            (switch Utilities|FlowControl|Switch|SwitchonE_SwticherCollisionType (Variables|Setting|ColliionBox|GetCollisionBoxType)
              (:NewEnumerator5
                (if (not (Variables|Setting|GetEnabled?)) :!label _label
                  (Variables|Setting|SetEnabled? true :!label _label_2)
                  (Traitement|OnServerEnableDisableLinkedLight true false :!label _label_3)))
              (:NewEnumerator0
                (Utilities|FlowControl|Sequence
                  (:then_0
                    (Utilities|FlowControl|RetriggerableDelay 0.1)
                    (Variables|Traitement|OnDelay|SetCanceled? false)
                    (Utilities|FlowControl|RetriggerableDelay (Variables|Setting|ColliionBox|GetKeepDuration))
                    (if (not (Variables|Traitement|OnDelay|GetCanceled?))
                      (Variables|Setting|SetEnabled? false)
                      (CallFunction|DoCollisionInteract)))
                  (:then_1
                    (goto _label_2))))
              (:NewEnumerator4
                (if (Variables|Setting|GetEnabled?)
                  (Variables|Setting|SetEnabled? false)
                  (goto _label_3)))
              (:NewEnumerator1
                (goto _label)))))))))

(event Custom|Multi_RefreshIndicatorLight
  (params (Enabled? :type Boolean))
  ;[1 1 1] (OnServer->Multi) Refresh indicator light
  (Rendering|Material|SetVectorParameterValue (Variables|Spawn|GetIndicatorLightMaterial) "Color" (select Enabled? "(R=0.000000,G=1.000000,B=0.000000,A=1.000000)" "(R=1.000000,G=0.000000,B=0.000000,A=1.000000)") :!class /Script/Engine.MaterialInstanceDynamic))

(event Custom|OnServer_RefreshIndicatorLight
  ;[1 1 1] (OnServer->Multi) Refresh indicator light
  (Networking|SwitchHasAuthority
    (:Authority
      (if (Utilities|Enum|Equal(Enum) (Variables|Setting|GetLightSwitchType) "NewEnumerator0")
        (CallFunction|MultiRefreshIndicatorLight (Variables|Setting|GetEnabled?))))))

(event Custom|OnServer_UpdateWidget
  ;[1 1 1] (OnServer -> Multi) Update the widget
  (Networking|SwitchHasAuthority
    (:Authority
      (if (and (Variables|Setting|Widget|GetShowWidget?) (Utilities|Enum|Equal(Enum) (Variables|Setting|GetLightSwitchType) "NewEnumerator0"))
        (CallFunction|MultiUpdateWidget (Variables|Setting|GetEnabled?))))))

(event Custom|OnServer_UpdateLightSwitch
  (params (ShowAction? :type Boolean))
  ;[1 1 1] (Server) Update (Called by LightSwitch)
  (Networking|SwitchHasAuthority
    (:Authority
      (Variables|Setting|SetEnabled? ShowAction?)
      (CallFunction|OnServerRefreshIndicatorLight)
      (Variables|Traitement|OnDelay|SetCanceled? true))))

(event Custom|DoCollisionInteract
  ;[1 1 1] (OnServer) Bengin/End overlap (Called by player collision)
  (Networking|SwitchHasAuthority
    (:Authority
      (Traitement|OnServerEnableDisableLinkedLight true false))))

(event Custom|Multi_UpdateWidget
  (params (Enabled? :type Boolean))
  ;[1 1 1] (OnServer -> Multi) Update the widget
  (bind _asw_interactive_name (Utilities|Casting|CastToW_InteractiveName (UserInterface|GetUserWidgetObject (Variables|Default|GetWidget))))
  (Default|UpdateWidget _asw_interactive_name (Variables|Traitement|byPlayer|GetInLineTrace?) (Traitement|GetWidgetText Enabled?)))

(event EventMSGLightonLinetraceChanged
  (params (InLinetrace? :type Boolean) (Key :type Text))
  ;[1 1 1] (Client) Actor are in the Player linetrace (Called by player)
  (Variables|Traitement|ByPlayer|SetActionKey Key)
  (if (Math|Boolean|NotEqual(Boolean) InLinetrace? (Variables|Traitement|byPlayer|GetInLineTrace?))
    (Variables|Traitement|byPlayer|SetInLineTrace? InLinetrace?)
    (if (Variables|Setting|Widget|GetShowWidget?)
      (bind _asw_interactive_name (Utilities|Casting|CastToW_InteractiveName (UserInterface|GetUserWidgetObject (Variables|Default|GetWidget))))
      (Default|UpdateWidget _asw_interactive_name (Variables|Traitement|byPlayer|GetInLineTrace?) (Traitement|GetWidgetText (Variables|Setting|GetEnabled?))))))

(event EventMSGLightSetOpacity
  (params (Show? :type Boolean) (PlayerRef :type Actor%20Object%20Reference) (Opacity :type Float%20%28single-precision%29))
  ;[1 1 1] (Client) Set Widget opacity (Called by component)
  (Traitement|RefreshWidgetOpacity Show? PlayerRef))

(event EventBeginPlay
  ;[1 1 1] Constructeur - Update all light and update widget if switcher
  (Utilities|FlowControl|Sequence
    (:then_0
      (Utilities|FlowControl|Delay 0.2)
      (Traitement|OnServerEnableDisableLinkedLight false true))
    (:then_1
      (if (and (Variables|Setting|Widget|GetShowWidget?) (Utilities|Enum|Equal(Enum) (Variables|Setting|GetLightSwitchType) "NewEnumerator0"))
        (bind _asw_interactive_name (Utilities|Casting|CastToW_InteractiveName (UserInterface|GetUserWidgetObject (Variables|Default|GetWidget))))
        (Default|StartUp _asw_interactive_name (Variables|Setting|Widget|GetLightSwitchName))))))

(fn ConstructionScript
  (bind _smlightswitchmovable (Variables|Setting|Mesh|GetSMLightSwitchMovable))
  (bind _smlightswitch (Variables|Setting|Mesh|GetSMLightSwitch))
  (bind _collisionbox (Variables|Default|GetCollisionBox))
  (Utilities|FlowControl|Sequence
    (:then_0
      ;[1 1 1] Refresh light switch and create indicator material (Everybody)
      (if (Utilities|Enum|Equal(Enum) (Variables|Setting|GetLightSwitchType) "NewEnumerator0")
        (bind _returnvalue (Rendering|Material|CreateDynamicMaterialInstance (Variables|Default|GetIndicatorLight) 0 "/Game/AntizeKitSystem/AntizeSystems/LightSystem/Resource/Materials/M_MasterEmissive.M_MasterEmissive" :!class /Script/Engine.PrimitiveComponent))
        (bind _output_get (Variables|Spawn|SetIndicatorLightMaterial _returnvalue))
        (Rendering|Material|SetScalarParameterValue _output_get "EmissivePower" 5e+01 :!class /Script/Engine.MaterialInstanceDynamic)
        (Rendering|Material|SetVectorParameterValue (Variables|Spawn|GetIndicatorLightMaterial) "Color" (select (Variables|Setting|GetEnabled?) "(R=0.000000,G=1.000000,B=0.000000,A=1.000000)" "(R=1.000000,G=0.000000,B=0.000000,A=1.000000)") :!class /Script/Engine.MaterialInstanceDynamic)
        (Rendering|Material|SetScalarParameterValue (Variables|Spawn|GetIndicatorLightMaterial) "UseFlickering?" 1.0 :!class /Script/Engine.MaterialInstanceDynamic)
        (Utilities|FlowControl|Sequence
          (:then_0
            ;[1 1 1] Disable widget if not enabled
            (if (not (Variables|Setting|Widget|GetShowWidget?))
              (Rendering|SetVisibility (Variables|Default|GetWidget) false false)))
          (:then_1
            ;[1 1 1] Disable indicator if not enabled
            (if (not (Variables|Setting|Mesh|GetShowIndicator?))
              (Rendering|SetVisibility (Variables|Default|GetIndicatorLight) false false)
              (Collision|SetCollisionEnabled (Variables|Default|GetIndicatorLight) "NoCollision")
              (else
                (Transformation|SetRelativeTransform (Variables|Default|GetIndicatorLight) (Variables|Setting|Mesh|GetIndicatorCorrection) false false)
                (Interact|ChangeLightSwitchMovable)))))))
    (:then_1
      ;[1 1 1] Disable component
      (if (Utilities|Enum|Equal(Enum) (Variables|Setting|GetLightSwitchType) "NewEnumerator1")
        (Rendering|SetVisibility (Variables|Default|GetLightSwitch) false false)
        (Collision|SetCollisionEnabled (Variables|Default|GetIndicatorLight) "NoCollision")
        (else
          (Rendering|SetVisibility _collisionbox false false)
          (Collision|SetCollisionEnabled _collisionbox "NoCollision"))))
    (:then_2
      ;[1 1 1] Setting up Static Mesh or Collision Box
      (if (Utilities|Enum|Equal(Enum) (Variables|Setting|GetLightSwitchType) "NewEnumerator0")
        (Transformation|SetRelativeTransform (Utilities|Select :Index (Variables|Setting|GetLightSwitchType) :NewEnumerator0 (Variables|Default|GetLightSwitch) :NewEnumerator1 (Variables|Default|GetCollisionBox)) (Variables|Setting|Mesh|GetSMCorrection) false false)
        (Transformation|SetRelativeTransform (Variables|Default|GetCollision) (Variables|Setting|Mesh|GetCollisionCorrection) false false)
        (Utilities|FlowControl|Sequence
          (:then_0
            (Components|StaticMesh|SetStaticMesh (Variables|Default|GetLightSwitchMovable) (select (Utilities|IsValid _smlightswitchmovable) _smlightswitchmovable "/Game/AntizeKitSystem/AntizeSystems/LightSystem/Resource/StaticMesh/SM_Empty.SM_Empty")))
          (:then_1
            (Components|StaticMesh|SetStaticMesh (Variables|Default|GetLightSwitch) (select (Utilities|IsValid _smlightswitch) _smlightswitch "/Game/AntizeKitSystem/AntizeSystems/LightSystem/Resource/StaticMesh/SM_Empty.SM_Empty"))))
        (else
          (Transformation|SetRelativeTransform (Variables|Default|GetCollisionBox) (Variables|Setting|ColliionBox|GetCollisionBoxCorrection) false false)
          (Components|StaticMesh|SetStaticMesh (Variables|Default|GetLightSwitch) "/Game/AntizeKitSystem/AntizeSystems/LightSystem/Resource/StaticMesh/SM_Empty.SM_Empty")
          (Components|StaticMesh|SetStaticMesh (Variables|Default|GetLightSwitchMovable) "/Game/AntizeKitSystem/AntizeSystems/LightSystem/Resource/StaticMesh/SM_Empty.SM_Empty"))))
    (:then_3
      ;[1 1 1] Clean linked array
      (for _array_element (Variables|Setting|GetLinkedLightSwitch)
        (if (!= _array_element self)
          (Utilities|Array|AddUnique (LocalVariables|GetLocal_Switcher) _array_element)))
      (Variables|Setting|SetLinkedLightSwitch (LocalVariables|GetLocal_Switcher))
      (for _array_element_2 (Variables|Setting|GetLinkedLight)
        (Utilities|Array|AddUnique (LocalVariables|GetLocal_Light) _array_element_2))
      (Variables|Setting|SetLinkedLight (LocalVariables|GetLocal_Light))
      (for _array_element_3 (Variables|Setting|GetLinkedInversedLight%20)
        (Utilities|Array|AddUnique (LocalVariables|GetLocal_InversedLight) _array_element_3))
      (Variables|Setting|SetLinkedInversedLight%20 (LocalVariables|GetLocal_InversedLight))
      ;[1 1 1] Refresh all switcher linked
      (if (Variables|Setting|GetRefreshLinkedSwitcher)
        (Variables|Setting|SetRefreshLinkedSwitcher false)
        (for _array_element_4 (Variables|Setting|GetLinkedLightSwitch)
          (CallFunction|OnServerUpdateLightSwitch _array_element_4 (Variables|Setting|GetEnabled?)))))))

(fn ChangeLightSwitchMovable
  ;[1 1 1] Update mesh if switcher
  (if (Utilities|Enum|Equal(Enum) (Variables|Setting|GetLightSwitchType) "NewEnumerator0")
    (bind _output_get (Variables|Traitement|SetMyFlipFlop (not (Variables|Traitement|GetMyFlipFlop))))
    (Transformation|SetRelativeRotation (Variables|Default|GetLightSwitchMovable) (Math|Rotator|MakeRotator 0.0 (select _output_get 1.8e+02 0.0) 0.0) false false)
    (return)
    (else
      (return))))

(fn GetWidgetText
  (params (Enabled? :type Boolean))
  (return (Utilities|Text|FormatText "\"{Action}\" {Message}" (Variables|Traitement|ByPlayer|GetActionKey) (select Enabled? "turn off" "turn on"))))

(fn RefreshWidgetOpacity
  (params (Show? :type Boolean) (PlayerRef :type Actor%20Object%20Reference))
  (bind _lightswitch (Variables|Default|GetLightSwitch))
  (bind _widget (Variables|Default|GetWidget))
  (bind _returnvalue (Transformation|GetWorldLocation _lightswitch))
  ;[1 1 1] Check if actor is in sight and set opacity
  (if (and (Variables|Setting|Widget|GetShowWidget?) (Utilities|Enum|Equal(Enum) (Variables|Setting|GetLightSwitchType) "NewEnumerator0"))
    (if Show?
      (bind _output_get (LocalVariables|SetLocal_PlayerRef PlayerRef))
      (LocalVariables|SetLocal_PlayerLocation (Transformation|GetActorLocation _output_get))
      (bind (_outhit _returnvalue_2) (Collision|LineTraceByChannel (LocalVariables|GetLocal_PlayerLocation) _returnvalue "TraceTypeQuery1" false (Utilities|Array|MakeArray (LocalVariables|GetLocal_PlayerRef)) "None" false "(R=0.000000,G=0.637930,B=1.000000,A=1.000000)" "(R=1.000000,G=0.000000,B=0.750000,A=1.000000)" 1e+01))
      (if _returnvalue_2
        (Rendering|SetVisibility _widget (== (.HitActor (Collision|BreakHitResult _outhit)) self) false)
        (if (== (.HitActor (Collision|BreakHitResult _outhit)) self)
          (Class|BPAntizeLightInterfaces|MSGLightSetOpacity(Message) (UserInterface|GetUserWidgetObject _widget) false 0 (Math|Float|Clamp(Float) (- 1.0 (/ (- (Math|Vector|VectorLength (- _returnvalue (LocalVariables|GetLocal_PlayerLocation))) (Variables|Setting|Widget|GetFadeStartDistance)) (Variables|Setting|Widget|GetFadeLength))))))
        (else
          (Rendering|SetVisibility (Variables|Default|GetWidget) false false)))
      (else
        (Rendering|SetVisibility (Variables|Default|GetWidget) false false)))))

(fn OnServerEnableDisableLinkedLight
  (params (RefreshLinkedSwitch? :type Boolean) (IsSpawnCall? :type Boolean))
  (bind _enabled_ (Variables|Setting|GetEnabled?))
  (bind _enabled__2 (Variables|Setting|GetEnabled?))
  (bind _returnvalue (not _enabled_))
  ;[1 1 1] Only on server
  (Networking|SwitchHasAuthority
    (:Authority
      (for _array_element (Variables|Setting|GetLinkedLight)
        (Utilities|IsValid _array_element
          (:Is%20Valid
            (if IsSpawnCall?
              (Default|ServerMySpawn _array_element _enabled__2 true true)
              (else
                (Default|LightInteract _array_element _enabled__2))))))
      (if (Variables|Setting|GetUseInversedLight?)
        (for _array_element_2 (Variables|Setting|GetLinkedInversedLight%20)
          (Utilities|IsValid _array_element_2
            (:Is%20Valid
              (if IsSpawnCall?
                (Default|ServerMySpawn _array_element_2 _returnvalue true true)
                (else
                  (Default|LightInteract _array_element_2 _returnvalue)))))))
      (if RefreshLinkedSwitch?
        (for _array_element_3 (Variables|Setting|GetLinkedLightSwitch)
          (Utilities|IsValid _array_element_3
            (:Is%20Valid
              (CallFunction|OnServerUpdateLightSwitch _array_element_3 (Variables|Setting|GetEnabled?)))))))))

(fn LightSwitchInteract
  (params (PlayerRef :type Character%20Object%20Reference))
  (bind _returnvalue (Actor|GetComponentbyClass PlayerRef "/Game/AntizeKitSystem/AntizeSystems/LightSystem/Blueprints/BP_LightComponent.BP_LightComponent_C"))
  ;[1 1 1] (Server) Interact (Called by player or collision)
  (Networking|SwitchHasAuthority
    (:Authority
      (Utilities|FlowControl|Sequence
        (:then_0
          (Variables|Setting|SetEnabled? (not (Variables|Setting|GetEnabled?)))
          (Interact|ChangeLightSwitchMovable)
          (CallFunction|OnServerRefreshIndicatorLight)
          (Utilities|FlowControl|Sequence
            (:then_0
              (Traitement|OnServerEnableDisableLinkedLight true false))
            (:then_1
              (CallFunction|OnServerUpdateWidget))))
        (:then_1
          (if (Utilities|Enum|Equal(Enum) (Variables|Setting|GetLightSwitchType) "NewEnumerator0")
            (Utilities|IsValid PlayerRef
              (:Is%20Valid
                (Utilities|IsValid _returnvalue
                  (:Is%20Valid
                    (Default|CallPlaySound _returnvalue "/Game/AntizeKitSystem/AntizeSystems/LightSystem/Resource/Sounds/Cue_Turn_Light.Cue_Turn_Light" (Transformation|GetActorLocation))))))))))))

(fn MSGLightGetCamera
  (return 0))