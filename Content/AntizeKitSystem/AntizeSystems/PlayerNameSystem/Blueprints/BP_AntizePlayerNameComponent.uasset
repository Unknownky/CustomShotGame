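; Pawn component that drives floating player-name widgets, including level changes and VoIP/writing state indicators.
; On the locally controlled pawn, a looping timer scans name-interface actors, applying team visibility rules, distance limits and line-of-sight traces to set each widget's opacity and scale locally.
; Server events clamp level changes and, after a retriggerable delay, call multicast events that refresh widgets and play effects through interface messages.
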(event Custom|Server_LevelUp
  (params (ActorRef :type Actor%20Object%20Reference))
  ;[1 1 1] Level up and level down
  (Variables|InGame|SetPlayerLevel (Math|Integer|Clamp(Integer) (+ (Variables|InGame|GetPlayerLevel) 1) 1 (Variables|InGame|GetMaxLevel)))
  (Utilities|FlowControl|RetriggerableDelay 0.1)
  (CallFunction|MultiPlayAnimandRefresh ActorRef "NewEnumerator0"))

(event Custom|Multi_PlayAnimAndRefresh
  (params (ActorRef :type Actor%20Object%20Reference) (EffectToPlay :type E_PlayerNameEffect%20Enum :default "NewEnumerator1"))
  ;[1 1 1] Level up and level down
  ;;[1 1 1] Refresh player infos on all players
  (bind _widgetref (Utilities|GetWidgetRef ActorRef)
    (:Is%20Valid
      (Class|BPAntizePlayerNameInterface|MSGAntizePNRefreshwidget(Message) _widgetref ActorRef)
      (Class|BPAntizePlayerNameInterface|MSGAntizePNPlayEffect(Message) _widgetref EffectToPlay))))

(event Custom|CheckForWidget
  ;[1 1 1] Loop check for NameWidget visibility
  (Utilities|IsOwnerValid
    (:Is%20Valid
      (Math|Integer|IncrementInt (Variables|Spawn|Others|GetAttempt)
        (:%20%20
          (bind _outactors (Actor|GetAllActorswithInterface "/Game/AntizeKitSystem/AntizeSystems/PlayerNameSystem/Blueprints/BP_AntizePlayerNameInterface.BP_AntizePlayerNameInterface_C"))
          (for _array_element _outactors
            (Utilities|IsValid _array_element
              (:Is%20Valid
                (bind _output_get (Variables|InGame|SetTempTarget _array_element))
                (if (!= _output_get (Variables|Spawn|Others|GetOwnerPawn))
                  ;;[1 1 1] Ensures the actor's infos are initialized before seeing the widget (OnlyOnce)
                  (Class|BPAntizePlayerNameInterface|MSGAntizePNTrytoInisitalize(Message) (Variables|InGame|GetTempTarget))
                  ;;[1 1 1] Remove the target for the collision to occur
                  (if (Variables|Settings|Visibility|GetIgnorePlayerObstacle?)
                    (bind _output_get_2 (Variables|InGame|SetTempActors _outactors))
                    (Utilities|Array|RemoveItem _output_get_2 (Variables|InGame|GetTempTarget)))
                  (Variables|InGame|SetActualDistance (Math|Vector|VectorLength (- (Transformation|GetActorLocation (Variables|InGame|GetTempTarget)) (Transformation|GetActorLocation (Variables|Spawn|Others|GetOwnerPawn)))))
                  (Utilities|ChoiceonTeamSettings
                    (:Default
                      (bind _viewlocation (Class|BPAntizePlayerNameInterface|MSGAntizePNGetViewLocation(Message) (Variables|Spawn|Others|GetOwnerPawn)))
                      (bind (_outhit _returnvalue) (Collision|LineTraceByChannel _viewlocation (Transformation|GetActorLocation (Variables|InGame|GetTempTarget)) (select (Variables|Settings|Visibility|GetIgnoreObstacle?) "TraceTypeQuery5" "TraceTypeQuery4") false (Variables|InGame|GetTempActors) "None"))
                      (if _returnvalue
                        (if (== (Variables|InGame|GetTempTarget) (.HitActor (Collision|BreakHitResult _outhit)))
                          (if (>= (Variables|Spawn|Others|GetAttempt) 30)
                            (CallFunction|FactoriseRefreshWidget (Variables|InGame|GetTempTarget)))
                          (CallFunction|SetWidgetScale)
                          (CallFunction|SetWidgetOpacity (Variables|InGame|GetTempTarget) (CallFunction|GetOpacity (Variables|InGame|GetActualDistance)))
                          (else
                            (CallFunction|SetWidgetOpacity (Variables|InGame|GetTempTarget) 0.0 :!label _label)))
                        (else
                          (goto _label))))
                    (:Hide
                      (CallFunction|SetWidgetOpacity (Variables|InGame|GetTempTarget) 0.0))
                    (:Show
                      (CallFunction|SetWidgetScale)
                      (CallFunction|SetWidgetOpacity (Variables|InGame|GetTempTarget) 1.0)))
                  (elif (>= (Variables|Spawn|Others|GetAttempt) 30)
                    (CallFunction|FactoriseRefreshWidget (Variables|Spawn|Others|GetOwnerPawn)))))))
          (if (>= (Variables|Spawn|Others|GetAttempt) 30)
            (Variables|Spawn|Others|SetAttempt 0)))))))

(event Custom|Server_LevelDown
  (params (ActorRef :type Actor%20Object%20Reference))
  ;[1 1 1] Level up and level down
  (Variables|InGame|SetPlayerLevel (Math|Integer|Clamp(Integer) (- (Variables|InGame|GetPlayerLevel) 1) 1 (Variables|InGame|GetMaxLevel)))
  (Utilities|FlowControl|RetriggerableDelay 0.1)
  (CallFunction|MultiPlayAnimandRefresh ActorRef "NewEnumerator0"))

(event Custom|Server_PlayState
  (params (ActorRef :type Actor%20Object%20Reference) (NewState :type E_PlayerVoiPWriteState%20Enum :default "NewEnumerator0"))
  ;[1 1 1] Play Write & VoiP State effect
  (Utilities|FlowControl|RetriggerableDelay 0.1)
  (CallFunction|MultiPlayState ActorRef NewState))

(event Custom|Multi_PlayState
  (params (ActorRef :type Actor%20Object%20Reference) (NewState :type E_PlayerVoiPWriteState%20Enum :default "NewEnumerator0"))
  ;[1 1 1] Play Write & VoiP State effect
  (bind _widgetref (Utilities|GetWidgetRef ActorRef)
    (:Is%20Valid
      (Class|BPAntizePlayerNameInterface|MSGAntizePNRefreshVOIPWriteState(Message) _widgetref NewState))))

(event Custom|Factorise_RefreshWidget
  (params (ActorRef :type Actor%20Object%20Reference))
  ;[1 1 1] Factorise RefreshWidget
  (bind _widgetref (Utilities|GetWidgetRef ActorRef)
    (:Is%20Valid
      (Class|BPAntizePlayerNameInterface|MSGAntizePNRefreshwidget(Message) _widgetref ActorRef))))

(event EventBeginPlay
  ;[1 1 1] Loop check for NameWidget visibility
  (bind _aspawn (Utilities|Casting|CastToPawn (Components|GetOwner) :!label _label)
    (:then
      (bind _output_get (Variables|Spawn|Others|SetOwnerPawn _aspawn))
      (Utilities|FlowControl|Sequence
        (:then_0
          (if (Pawn|IsLocallyControlled _output_get)
            (bind _returnvalue (Utilities|Time|SetTimerbyEvent (delegate Custom|CheckForWidget) 0.1 true))
            (Variables|Spawn|SetTimer_CheckForLoop _returnvalue)
            (CallFunction|FactoriseRefreshWidget (Variables|Spawn|Others|GetOwnerPawn))
            (if (Variables|Settings|GetShowOwnPlayerName?)
              (CallFunction|SetWidgetOpacity (Variables|Spawn|Others|GetOwnerPawn) 1.0)
              (else
                (CallFunction|SetWidgetOpacity (Variables|Spawn|Others|GetOwnerPawn) 0.0)))))
        (:then_1
          (bind _widgetref (Utilities|GetWidgetRef (Variables|Spawn|Others|GetOwnerPawn))
            (:Is%20Valid
              (bind _asw_player_name (Utilities|Casting|CastToW_PlayerName _widgetref))
              (Default|ShowHideRank _asw_player_name (Variables|Settings|GetShowRank?)))))))
    (:CastFailed
      (Utilities|FlowControl|Delay 0.2)
      (goto _label))))

(fn GetOpacity
  (params (Distance :type Float%20%28single-precision%29))
  (bind _distancetostartfade (Variables|Settings|Visibility|GetDistanceToStartFade))
  (if (>= (Variables|Settings|Visibility|GetDistanceToStartFade) Distance)
    (return 1.0)
    (else
      (return (Math|Float|Lerp 1.0 0.0 (Math|Float|Clamp(Float) (/ (- Distance _distancetostartfade) (- (Variables|Settings|Visibility|GetMaxDistanceWidget) _distancetostartfade))))))))

(fn SetWidgetScale
  (bind _maxwidgetscale (Variables|Settings|Widget|GetMaxWidgetScale))
  (bind _actualdistance (Variables|InGame|GetActualDistance))
  (bind _minwidgetscale (Variables|Settings|Widget|GetMinWidgetScale))
  (bind _distancetostartscale (Variables|Settings|Widget|GetDistanceToStartScale))
  (bind _maxdistancescale (Variables|Settings|Widget|GetMaxDistanceScale))
  (bind _returnvalue (- _actualdistance _distancetostartscale))
  (bind _returnvalue_2 (- _maxdistancescale _distancetostartscale))
  (bind _returnvalue_3 (/ _returnvalue _returnvalue_2))
  (bind _returnvalue_4 (Math|Float|Clamp(Float) _returnvalue_3))
  (bind _returnvalue_5 (Math|Float|Lerp _maxwidgetscale _minwidgetscale _returnvalue_4))
  ;[1 1 1] Set widget scale (Local)
  (bind _widgetref (Utilities|GetWidgetRef (Variables|InGame|GetTempTarget))
    (:Is%20Valid
      (bind _asw_player_name (Utilities|Casting|CastToW_PlayerName _widgetref)
        (:then
          (if (!= (Variables|/Script/UMG.ScaleBox|GetUserSpecifiedScale (Variables|/Game/AntizeKitSystem/AntizeSystems/PlayerNameSystem/Widgets/W_PlayerName.W_PlayerName_C|GetMyScaleBox _asw_player_name)) _returnvalue_5)
            (Class|ScaleBox|SetUserSpecifiedScale (Variables|/Game/AntizeKitSystem/AntizeSystems/PlayerNameSystem/Widgets/W_PlayerName.W_PlayerName_C|GetMyScaleBox _asw_player_name) _returnvalue_5)
            (return)
            (else
              (return))))
        (:CastFailed
          _)))
    (:NotValid
      _))
  (return))

(fn SetWidgetOpacity
  (params (PlayerRef :type Actor%20Object%20Reference) (NewOpacity :type Float%20%28single-precision%29))
  ;[1 1 1] Set widget opacity (Local)
  (bind _widgetref (Utilities|GetWidgetRef PlayerRef)
    (:Is%20Valid
      (if (!= (Class|Widget|GetRenderOpacity _widgetref) NewOpacity)
        (Widget|SetRenderOpacity _widgetref NewOpacity)))
    (:NotValid
      _))
  (return))

(fn GetinSameTeam
  (bind _teamid (Class|BPAntizeChatInterface|MSGGetTeamID(Message) (Variables|Spawn|Others|GetOwnerPawn)))
  (if (>= _teamid 0)
    (bind _teamid_2 (Class|BPAntizeChatInterface|MSGGetTeamID(Message) (Variables|InGame|GetTempTarget)))
    (return (== _teamid_2 _teamid))
    (else
      (return false))))

(fn MSGAntizePNGetLevel
  (return (Variables|InGame|GetPlayerLevel)))

(fn MSGAntizePNGetPlayerNameComponent
  (return 0))

(fn MSGAntizePNGetViewLocation
  (return "0, 0, 0"))

(fn MSGAntizePNGetWidgetRef
  (return 0))

(fn MSGAntizePNTrytoInisitalize)