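; BP_Portalwall is a wall actor that hosts portals, with its plane scaled from wall width and height in the construction script.
; A placement request converts the position to wall-local space, runs it through a bounds-clamping helper, and rejects it if a 2D rectangle test overlaps an existing portal.
; Accepted requests spawn BP_传送门 aligned to the wall and track it in PortalsOnWall until its destroy event removes it.
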(event EventBeginPlay)

(event Collision|EventActorBeginOverlap
  (params (OtherActor :type Actor%20Object%20Reference)))

(event EventTick
  (params (DeltaSeconds :type Float%20%28single-precision%29)))

(fn ConstructionScript
  (Transformation|SetWorldScale3D (Variables|Default|GetPlane) (Math|Vector|MakeVector (/ (Variables|Default|Getwallhight) 1e+02) (/ (Variables|Default|Getwallwidth) 1e+02) 1.0)))

(fn 尝试添加传送门
  (params (portalOrigin :type Vector) (Portal%20A :type Boolean))
  (LocalVariables|SetRelativePortalOrigin (Math|Transform|InverseTransformLocation (Transformation|GetActorTransform) portalOrigin))
  (bind (_clampedy _clampedz) (CallFunction|将传送门约束到墙 (.y (LocalVariables|GetRelativePortalOrigin)) (.z (LocalVariables|GetRelativePortalOrigin))))
  (LocalVariables|SetRelativePortalOrigin (Math|Vector|MakeVector (.x (LocalVariables|GetRelativePortalOrigin)) _clampedy _clampedz))
  (if (CallFunction|有新门户的空间吗？ (.y (LocalVariables|GetRelativePortalOrigin)) (.z (LocalVariables|GetRelativePortalOrigin)))
    (bind _returnvalue (Game|SpawnActorfromClass "/Game/传送门/BP_传送门.BP_传送门_C" (Math|Transform|MakeTransform (Math|Transform|TransformLocation (Transformation|GetActorTransform) (LocalVariables|GetRelativePortalOrigin)) (Transformation|GetActorRotation) "1.000000,1.000000,1.000000") "Undefined" 0 Portal%20A 0))
    (Utilities|Array|Add (Variables|Default|GetPortalsOnWall) _returnvalue)
    (Game|BindEventtoOnDestroyed _returnvalue (EventDispatchers|CreateEvent :!event 传送门被销毁))
    (return _returnvalue)))

(fn 将传送门约束到墙
  (params (PortalY :type Float%20%28double-precision%29) (PortalZ :type Float%20%28double-precision%29))
  (bind _returnvalue (CallFunction|限制点在墙的位置 PortalY (Variables|Default|Getwallwidth) 0.0))
  (LocalVariables|SetClamped_Y _returnvalue)
  (bind _returnvalue_2 (CallFunction|限制点在墙的位置 PortalZ (Variables|Default|Getwallwidth) 0.0))
  (LocalVariables|SetClamped_Z _returnvalue_2)
  (return (LocalVariables|GetClamped_Y) (LocalVariables|GetClamped_Z)))

(fn 限制点在墙的位置
  (params (point :type Float%20%28double-precision%29) (WallSize :type Float%20%28double-precision%29) (PortalRadius :type Float%20%28double-precision%29))
  (LocalVariables|SetOffset (Math|Float|Clamp(Float) (- (- (/ WallSize 0.0) PortalRadius) (Math|Float|Absolute(Float) point)) -1e+41 0.0))
  (LocalVariables|SetOffset (select (< point 0.0) 1.0 -1.0))
  (return (- point (LocalVariables|GetOffset))))

(fn 传送门被销毁
  (params (传送门 :type Actor%20Object%20Reference))
  (Utilities|Array|RemoveItem (Variables|Default|GetPortalsOnWall) 传送门))

(fn 有新门户的空间吗？
  (params (NewPortalY :type Float%20%28double-precision%29) (NewPortalZ :type Float%20%28double-precision%29))
  (bind (_radiusy _radiusz) (Utilities|PortalSize))
  (bind _returnvalue (Math|Vector2D|MakeVector2D _radiusy _radiusz))
  (for _array_element (Variables|Default|GetPortalsOnWall)
    (bind _colliding_ (CallFunction|RecttoRectCollision (Math|Vector2D|MakeVector2D (.y (Math|Transform|InverseTransformLocation (Transformation|GetActorTransform) (Transformation|GetActorLocation _array_element))) (.z (Math|Transform|InverseTransformLocation (Transformation|GetActorTransform) (Transformation|GetActorLocation _array_element)))) _returnvalue (Math|Vector2D|MakeVector2D NewPortalY NewPortalZ) _returnvalue))
    (if _colliding_
      (return false)))
  (return true))